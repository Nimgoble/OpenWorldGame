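; Player state for the Easy Building System that gives each player a test name and relays door lock actions.
; On BeginPlay, the authority builds the name from the game state's player count, then increments that count.
; Interface events forward to custom events that call the lock to set a password, authorize a player or create the code lock widget.
; An interface getter exposes the test name.
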(event Custom|SetDoorLockPassword
  (params (DoorLock :type BP%20EBS%20Door%20Lock%20Object%20Reference) (Password :type Text) (PlayerName :type String))
  ;[1 1 1] Door lock events.
  (Default|SetPassword DoorLock Password PlayerName))

(event Custom|CreateCodeLockWidget
  (params (CodeLock :type BP%20EBS%20Code%20Lock%20Object%20Reference) (Pawn :type Pawn%20Object%20Reference))
  ;[1 1 1] Door lock events.
  (Default|CreateLockWidget CodeLock Pawn))

(event Custom|AutorizeDoorLock
  (params (DoorLock :type BP%20EBS%20Door%20Lock%20Object%20Reference) (PlayerName :type String))
  ;[1 1 1] Door lock events.
  (Default|Autorize DoorLock PlayerName))

(event EventBeginPlay
  ;[1 1 1] Players gets unique name.
  (Networking|SwitchHasAuthority
    (:Authority
      (bind _asbp_ebs_game_state (Utilities|Casting|CastToBP_EBS_GameState (Game|GetGameState)))
      (Variables|Default|SetTestPlayerName (Utilities|String|ToString(Text) (Utilities|Text|FormatText "Player {0}" (Variables|/Game/EasyBuildingSystem/Blueprints/Game/BP_EBS_GameState.BP_EBS_GameState_C|GetPlayerCount _asbp_ebs_game_state))))
      (Math|Integer|IncrementInt (Variables|/Game/EasyBuildingSystem/Blueprints/Game/BP_EBS_GameState.BP_EBS_GameState_C|GetPlayerCount _asbp_ebs_game_state)))))

(event EventCreateCodeLockWidgetBPI
  (params (CodeLock :type BP%20EBS%20Code%20Lock%20Object%20Reference) (Pawn :type Pawn%20Object%20Reference))
  ;[1 1 1] Door lock events.
  (CallFunction|CreateCodeLockWidget CodeLock Pawn))

(event EventSetDoorLockPasswordBPI
  (params (DoorLock :type BP%20EBS%20Door%20Lock%20Object%20Reference) (Password :type Text) (PlayerName :type String))
  ;[1 1 1] Door lock events.
  (CallFunction|SetDoorLockPassword DoorLock Password PlayerName))

(event EventAutorizeDoorLockBPI
  (params (DoorLock :type BP%20EBS%20Door%20Lock%20Object%20Reference) (PlayerName :type String))
  ;[1 1 1] Door lock events.
  (CallFunction|AutorizeDoorLock DoorLock PlayerName))

(fn ConstructionScript)

(fn GetTestPlayerNameBPI
  (return (Variables|Default|GetTestPlayerName)))