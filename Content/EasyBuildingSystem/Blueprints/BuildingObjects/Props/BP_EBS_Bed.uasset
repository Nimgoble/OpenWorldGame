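; BP_EBS_Bed is a placeable bed prop in the Easy Building System that players can claim or unclaim with E.
; Use toggles the player's name in ClaimedPlayers, which drives the prompt text and is reported with ClaimedDistance through GetClaimInfo.
; Save and load overrides extend the parent to persist claims in BP_EBS_GameSave by SaveID.
; For placement, it supplies four floor checkers and tests BuildCollision with landscape included.
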(event Custom|ClaimUnclaim
  (params (PlayerName :type String))
  (bind _claimedplayers (Variables|State|GetClaimedPlayers))
  ;[1 1 1] Claim or Unclaim for characters player.
  (if (Utilities|Array|ContainsItem _claimedplayers PlayerName)
    (Utilities|Array|RemoveItem _claimedplayers PlayerName)
    (else
      (Utilities|Array|AddUnique _claimedplayers PlayerName))))

(event EventUse
  (params (Pawn :type Pawn%20Object%20Reference) (Key :type Key%20Structure))
  ;[1 1 1] Claim or Unclaim for characters player.
  (if (== Key "E")
    (CallFunction|ClaimUnclaim (PlayerState|GetPlayerName (Variables|/Script/Engine.Pawn|GetPlayerState Pawn)))
    (else
      (|CallParentFunction Pawn Key))))

(event EventSetFloorCheckers
  ;[1 1 1] Overrided Events.
  (Variables|Default|SetFloorCheckers (Utilities|Array|MakeArray (Variables|Default|GetFloorChecker1) (Variables|Default|GetFloorChecker2) (Variables|Default|GetFloorChecker3) (Variables|Default|GetFloorChecker4))))

(event EventDestroyBuildComponents
  ;[1 1 1] Overrided Events.
  (Components|DestroyComponent (Variables|Default|GetBuildCollision)))

(fn ConstructionScript
  (|CallParentFunction))

(fn GetUsableText
  (params (Pawn :type Pawn%20Object%20Reference))
  (if (not (Utilities|Array|ContainsItem (Variables|State|GetClaimedPlayers) (PlayerState|GetPlayerName (Variables|/Script/Engine.Pawn|GetPlayerState Pawn))))
    (return "[E] Claim.")
    (else
      (return "[E] Unclaim."))))

(fn LoadDataBPI
  (params (SaveData :type Save%20Game%20Object%20Reference))
  (bind _success (|CallParentFunction SaveData))
  (if _success
    (Variables|State|SetClaimedPlayers (Utilities|Struct|BreakSTR_EBS_ClaimData (.Value (Utilities|Map|Find (Variables|/Game/EasyBuildingSystem/Blueprints/Game/SaveData/BP_EBS_GameSave.BP_EBS_GameSave_C|GetSavedClaimsData (.AsBP%20EBS%20Game%20Save (Utilities|Casting|CastToBP_EBS_GameSave SaveData))) (Variables|Default|GetSaveID)))))
    (return true)
    (else
      (return false))))

(fn SaveDataBPI
  (params (SaveData :type Save%20Game%20Object%20Reference))
  (bind _success (|CallParentFunction SaveData))
  (if _success
    (Utilities|Map|Add (Variables|/Game/EasyBuildingSystem/Blueprints/Game/SaveData/BP_EBS_GameSave.BP_EBS_GameSave_C|GetSavedClaimsData (.AsBP%20EBS%20Game%20Save (Utilities|Casting|CastToBP_EBS_GameSave SaveData))) (Variables|Default|GetSaveID) (Utilities|Struct|MakeSTR_EBS_ClaimData (Variables|State|GetClaimedPlayers)))
    (return true)
    (else
      (return false))))

(fn CheckBuildCollisions
  (params (Actor :type Actor%20Object%20Reference))
  (return (CallFunction|CheckActorCollisions Actor (Variables|Default|GetBuildCollision) false)))

(fn GetClaimInfo
  (bind _claimedplayers (Variables|State|GetClaimedPlayers))
  (return (> (Utilities|Array|Length _claimedplayers) 0) _claimedplayers (Variables|State|GetClaimedDistance)))