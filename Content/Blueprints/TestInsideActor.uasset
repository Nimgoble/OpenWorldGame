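; Test actor that checks whether one referenced actor, Test1, lies inside another, Test2, and prints the results.
; On BeginPlay it runs IsActorInsideActor on colliding components only, then IsComponentInsideComponent between Test1's BuildCollision and Test2's Collision.
; Each check prints a formatted text naming both objects and saying whether the first is inside the second.
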(event EventBeginPlay
  (bind _test1 (Variables|Default|GetTest1))
  (bind _test2 (Variables|Default|GetTest2))
  (bind _buildcollision (Variables|/Game/EasyBuildingSystem/Blueprints/BuildingObjects/Base/BP_EBS_Foundation.BP_EBS_Foundation_C|GetBuildCollision _test1))
  (bind _collision (Variables|/Game/EasyBuildingSystem/Blueprints/BuildingObjects/Props/CampArea.CampArea_C|GetCollision _test2))
  (bind _returnvalue (Utilities|GetDisplayName _buildcollision))
  (bind _returnvalue_2 (Utilities|GetDisplayName _collision))
  (bind _returnvalue_3 (Class|OWGBlueprintFunctionLibrary|IsActorInsideActor _test1 _test2 true))
  (if _returnvalue_3
    (Development|PrintText (Utilities|Text|FormatText "{0} is inside {1}" (Utilities|GetDisplayName _test1) (Utilities|GetDisplayName _test2)))
    (else
      (Development|PrintText (Utilities|Text|FormatText "{0} is NOT inside {1}" (Utilities|GetDisplayName _test1) (Utilities|GetDisplayName _test2)))))
  (bind _returnvalue_4 (Class|OWGBlueprintFunctionLibrary|IsComponentInsideComponent _buildcollision _collision))
  (if _returnvalue_4
    (Development|PrintText (Utilities|Text|FormatText "{0} is inside {1}" _returnvalue _returnvalue_2))
    (else
      (Development|PrintText (Utilities|Text|FormatText "{0} is NOT inside {1}" _returnvalue _returnvalue_2)))))

(event Collision|EventActorBeginOverlap
  (params (OtherActor :type Actor%20Object%20Reference)))

(event EventTick
  (params (DeltaSeconds :type Float%20%28single-precision%29)))

(fn ConstructionScript)