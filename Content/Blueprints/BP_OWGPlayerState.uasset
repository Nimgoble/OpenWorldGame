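; BP_OWGPlayerState is a player state Blueprint that starts a player camp query once the server has the player's PlayFab ID.
; When the ServerPlayFabIdSet event fires with a non-empty ID, it casts its owner to OWGPlayerController and calls QueryPlayerCamp.
; The SetPlayFabID function is empty, and the construction script only calls its parent.
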(event EventBeginPlay
  (|CallParentFunction) ; This node is disabled and will not be called.\nDrag off pins to build functionality.
)

(event EventTick
  (params (DeltaSeconds :type Float%20%28single-precision%29)))

(event EventServerPlayFabIdSet
  (if (not (Utilities|Array|IsEmpty (Class|OWGPlayerState|GetPlayFabId)))
    (bind _asowgplayer_controller (Utilities|Casting|CastToOWGPlayerController (Components|GetOwner)))
    (Default|QueryPlayerCamp _asowgplayer_controller)))

(fn ConstructionScript
  (|CallParentFunction))

(fn SetPlayFabID
  (params (PlayFabID :type String)))