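; Blueprint helper library that converts camp data and its building objects to and from JSON, with small utilities for landscape detection, struct conversion and JSON wrapping.
; Camp functions compose the building and transform converters, storing rotation as three axis vectors.
; Deserialization always resets scale to one and marks camp data valid, even for invalid JSON.
; A location of -1 on all axes marks an invalid camp transform.
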(fn IsLandscape
  (params (Actor :type Actor%20Object%20Reference))
  (return (or (Utilities|Array|ContainsItem (LocalVariables|GetLandscapeTypes) (Utilities|GetClass Actor)) (Actor|ActorHasTag Actor "IsLandscape"))))

(fn ToBuildingObject
  (params (Old :type STR%20EBS%20Object%20Data%20Structure))
  (bind (_id _class _transform _durability _floor) (Utilities|Struct|BreakSTR_EBS_ObjectData Old))
  (return (Utilities|Struct|MakeBuildingObject _id _transform _durability _floor)))

(fn SerializeCamp
  (params (Camp :type Camp%20Data%20Structure))
  (bind (_transform _buildingobjects) (Utilities|Struct|BreakCampData Camp))
  (bind _jsonbuildingobjects (LocalVariables|GetJsonBuildingObjects))
  (bind _output_get (LocalVariables|SetRoot (Class|PlayFabJsonObject|ConstructJsonObject)))
  (for _array_element _buildingobjects
    (bind _out (CallFunction|SerializeBuildingObject _array_element (LocalVariables|Get__WorldContext)))
    (Utilities|Array|Add _jsonbuildingobjects _out))
  (Class|PlayFabJsonObject|SetObjectArrayField _output_get "BuildingObjects" _jsonbuildingobjects)
  (bind _out_2 (CallFunction|SerializeTransform _transform))
  (Class|PlayFabJsonObject|SetObjectField _output_get "Transform" _out_2)
  (return _output_get))

(fn SerializeBuildingObject
  (params (In :type Building%20Object%20Structure))
  (bind (_id _transform _durability _floor) (Utilities|Struct|BreakBuildingObject In))
  (bind (_location _rotation) (Math|Transform|BreakTransform _transform))
  (bind (_x _y _z) (Math|Rotator|BreakRotIntoAxes _rotation))
  (bind (_x_2 _y_2 _z_2) (Math|Vector|BreakVector _location))
  (bind (_x_3 _y_3 _z_3) (Math|Vector|BreakVector _z))
  (bind (_x_4 _y_4 _z_4) (Math|Vector|BreakVector _x))
  (bind (_x_5 _y_5 _z_5) (Math|Vector|BreakVector _y))
  (bind _output_get (LocalVariables|SetBuildingJson (Class|PlayFabJsonObject|ConstructJsonObject)))
  (Class|PlayFabJsonObject|SetStringField _output_get "ID" (Utilities|String|ToString(Name) _id))
  (Class|PlayFabJsonObject|SetNumberField _output_get "Durability" _durability)
  (Class|PlayFabJsonObject|SetNumberField _output_get "Floor" (Math|Conversions|ToFloat(Integer) _floor))
  ;[1 1 1] Transform
  (bind _output_get_2 (LocalVariables|SetTransform (Class|PlayFabJsonObject|ConstructJsonObject)))
  ;;[1 1 1] Location
  (Class|PlayFabJsonObject|SetNumberArrayField _output_get_2 "Location" (Utilities|Array|MakeArray _x_2 _y_2 _z_2))
  ;;[1 1 1] Rotation
  (bind _output_get_3 (LocalVariables|SetRotation (Class|PlayFabJsonObject|ConstructJsonObject)))
  (Class|PlayFabJsonObject|SetNumberArrayField _output_get_3 "X" (Utilities|Array|MakeArray _x_4 _y_4 _z_4))
  (Class|PlayFabJsonObject|SetNumberArrayField _output_get_3 "Y" (Utilities|Array|MakeArray _x_5 _y_5 _z_5))
  (Class|PlayFabJsonObject|SetNumberArrayField _output_get_3 "Z" (Utilities|Array|MakeArray _x_3 _y_3 _z_3))
  (Class|PlayFabJsonObject|SetObjectField _output_get_2 "Rotation" _output_get_3)
  (Class|PlayFabJsonObject|SetObjectField _output_get "Transform" _output_get_2)
  (return (LocalVariables|GetBuildingJson)))

(fn WrapJson
  (params (FieldName :type String) (Json :type Play%20Fab%20Json%20Object%20Object%20Reference) (StringifyObject :type Boolean))
  (bind _output_get (LocalVariables|SetRoot (Class|PlayFabJsonObject|ConstructJsonObject)))
  (if StringifyObject
    (Class|PlayFabJsonObject|SetStringField _output_get FieldName (Class|PlayFabJsonObject|EncodeJson Json))
    (else
      (Class|PlayFabJsonObject|SetObjectField _output_get FieldName Json)))
  (return (LocalVariables|GetRoot)))

(fn DeserializeCamp
  (params (CampJSON :type Play%20Fab%20Json%20Object%20Object%20Reference))
  (bind _buildingobjects (LocalVariables|GetBuildingObjects))
  (Utilities|IsValid CampJSON
    (:Is%20Valid
      (bind _out (CallFunction|DeserializeTransform (Class|PlayFabJsonObject|GetObjectField CampJSON "Transform")))
      (bind _returnvalue (Class|PlayFabJsonObject|GetObjectArrayField CampJSON "BuildingObjects"))
      (for _array_element _returnvalue
        (bind _buildingobject (CallFunction|DeserializeBuildingObject _array_element))
        (Utilities|Array|Add _buildingobjects _buildingobject))
      (return (Utilities|Struct|MakeCampData _out _buildingobjects true)))
    (:Is%20Not%20Valid
      (return (Utilities|Struct|MakeCampData "-1.000000,-1.000000,-1.000000|0.000000,0.000000,0.000000|1.000000,1.000000,1.000000" 0 true)))))

(fn DeserializeBuildingObject
  (params (BuildingObjectJSON :type Play%20Fab%20Json%20Object%20Object%20Reference))
  (bind _out (CallFunction|DeserializeTransform (Class|PlayFabJsonObject|GetObjectField BuildingObjectJSON "Transform")))
  (return (Utilities|Struct|MakeBuildingObject (Utilities|String|StringToName (Class|PlayFabJsonObject|GetStringField BuildingObjectJSON "ID")) _out (Class|PlayFabJsonObject|GetNumberField BuildingObjectJSON "Durability") (Math|Float|Truncate (Class|PlayFabJsonObject|GetNumberField BuildingObjectJSON "Floor")))))

(fn NumberArraytoVector
  (params (In :type Array%20of%20Floats%20%28single-precision%29))
  (return (Math|Vector|MakeVector (Utilities|Array|Get(acopy) In) (Utilities|Array|Get(acopy) In 1) (Utilities|Array|Get(acopy) In 2))))

(fn DeserializeTransform
  (params (In :type Play%20Fab%20Json%20Object%20Object%20Reference))
  (bind _returnvalue (Class|PlayFabJsonObject|GetObjectField In "Rotation"))
  (bind _returnvalue_2 (Class|PlayFabJsonObject|GetNumberArrayField In "Location"))
  (bind _out (CallFunction|NumberArraytoVector _returnvalue_2))
  (bind _returnvalue_3 (Class|PlayFabJsonObject|GetNumberArrayField _returnvalue "X"))
  (bind _out_2 (CallFunction|NumberArraytoVector _returnvalue_3))
  (bind _returnvalue_4 (Class|PlayFabJsonObject|GetNumberArrayField _returnvalue "Y"))
  (bind _out_3 (CallFunction|NumberArraytoVector _returnvalue_4))
  (bind _returnvalue_5 (Class|PlayFabJsonObject|GetNumberArrayField _returnvalue "Z"))
  (bind _out_4 (CallFunction|NumberArraytoVector _returnvalue_5))
  (return (Math|Transform|MakeTransform _out (Math|Rotator|MakeRotationfromAxes _out_2 _out_3 _out_4))))

(fn SerializeTransform
  (params (Transform :type Transform))
  (bind (_location _rotation _scale) (Math|Transform|BreakTransform Transform))
  (bind (_x _y _z) (Math|Rotator|BreakRotIntoAxes _rotation))
  (bind _output_get (LocalVariables|SetReturnValue (Class|PlayFabJsonObject|ConstructJsonObject)))
  ;[1 1 1] Location
  (bind _out (CallFunction|VectortoNumberArray _location))
  (Class|PlayFabJsonObject|SetNumberArrayField _output_get "Location" _out)
  ;[1 1 1] Scale
  (bind _out_2 (CallFunction|VectortoNumberArray _scale))
  (Class|PlayFabJsonObject|SetNumberArrayField _output_get "Scale" _out_2)
  ;[1 1 1] Rotation
  (bind _output_get_2 (LocalVariables|SetRotation (Class|PlayFabJsonObject|ConstructJsonObject)))
  (bind _out_3 (CallFunction|VectortoNumberArray _x))
  (Class|PlayFabJsonObject|SetNumberArrayField _output_get_2 "X" _out_3)
  (bind _out_4 (CallFunction|VectortoNumberArray _y))
  (Class|PlayFabJsonObject|SetNumberArrayField _output_get_2 "Y" _out_4)
  (bind _out_5 (CallFunction|VectortoNumberArray _z))
  (Class|PlayFabJsonObject|SetNumberArrayField _output_get_2 "Z" _out_5)
  (Class|PlayFabJsonObject|SetObjectField _output_get "Rotation" _output_get_2)
  (return _output_get))

(fn VectortoNumberArray
  (params (In :type Vector))
  (bind (_x _y _z) (Math|Vector|BreakVector In))
  (return (Utilities|Array|MakeArray _x _y _z)))

(fn IsValidCampTransform
  (params (In :type Transform))
  (bind _location (Math|Transform|BreakTransform In))
  (bind (_x _y _z) (Math|Vector|BreakVector _location))
  (return (not (Math|Boolean|ANDBoolean (== _x -1.0) (== _y -1.0) (== _z -1.0)))))