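; Base Blueprint for interactable items in the RPG inventory system, with empty stubs for interaction, end interaction, removal and game load events.
; On Initialize, it hands its interactable area, interaction widget and both meshes as highlightable objects to the ACInteractable component.
; The construction script shows the skeletal mesh only when no valid static mesh is assigned.
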(event EventInteraction
  ;[0 0 0 0.227 22] On Interaction
)

(event EventEndInteraction
  ;[0 0 0 0.227 22] On End Interaction
)

(event EventInitialize
  ;[0 0 0 0.227 22] On Initialize
  (Default|SetupInteractableReferences (Variables|Default|GetAC_Interactable) (Variables|Default|GetInteractableArea) (Variables|Default|GetInteractionWidget) (Utilities|Set|MakeSet (Variables|Default|GetStaticMesh) (Variables|Default|GetSkeletalMesh))))

(event EventRemoveInteraction
  ;[0 0 0 0.227 22] On Remove Interaction
)

(event EventGameLoad
  ;[0 0 0 0.227 22] On Game Load
)

(fn ConstructionScript
  (Rendering|SetVisibility (Variables|Default|GetSkeletalMesh) (select (Utilities|IsValid (Variables|/Script/Engine.StaticMeshComponent|GetStaticMesh (Variables|Default|GetStaticMesh))) false true) false))