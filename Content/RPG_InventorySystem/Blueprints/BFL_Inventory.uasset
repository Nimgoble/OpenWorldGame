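; Blueprint function library of shared helpers for the RPG inventory system.
; Getters fetch the player character and its inventory, crafting, interaction, leveling and consumable components, backing UI-open, interactable and EXP helpers.
; Array utilities filter items by type or sort them by type and rarity through bucketing, by value and weight through descending insertion, or simply drop invalid entries.
; Other helpers check pause via near-zero time dilation, map gamepad icons and play UI sounds.
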(fn GetACInventory
  (bind _returnvalue (Game|GetPlayerCharacter 0))
  (bind _returnvalue_2 (Actor|GetComponentbyClass _returnvalue "/Game/RPG_InventorySystem/Blueprints/Components/AC_Inventory.AC_Inventory_C"))
  (Utilities|IsValid _returnvalue_2
    (:Is%20Valid
      (return _returnvalue_2))))

(fn GetPlayerReference
  (bind _asbp_rpginventory_character (Utilities|Casting|CastToBP_RPGInventoryCharacter (Game|GetPlayerCharacter 0)))
  (return _asbp_rpginventory_character))

(fn GetACCrafting
  (bind _returnvalue (Game|GetPlayerCharacter 0))
  (bind _returnvalue_2 (Actor|GetComponentbyClass _returnvalue "/Game/RPG_InventorySystem/Blueprints/Components/AC_Crafting.AC_Crafting_C"))
  (Utilities|IsValid _returnvalue_2
    (:Is%20Valid
      (return _returnvalue_2))))

(fn IsUIOpen?
  (bind _ac_inventory (CallFunction|GetACInventory))
  (bind _ac_crafting (CallFunction|GetACCrafting))
  (if (Math|Boolean|ORBoolean (Variables|/Game/RPG_InventorySystem/Blueprints/Components/AC_Inventory.AC_Inventory_C|GetIsInventoryOpen? _ac_inventory) (Variables|/Game/RPG_InventorySystem/Blueprints/Components/AC_Inventory.AC_Inventory_C|GetIsItemsBarOpen? _ac_inventory) (Variables|/Game/RPG_InventorySystem/Blueprints/Components/AC_Inventory.AC_Inventory_C|GetIs%20Vendor/Storage%20Open? _ac_inventory) (Variables|/Game/RPG_InventorySystem/Blueprints/Components/AC_Inventory.AC_Inventory_C|GetIs%20LoadGameWindow%20Open? _ac_inventory) (Variables|/Game/RPG_InventorySystem/Blueprints/Components/AC_Crafting.AC_Crafting_C|GetIs%20Crafting%20Open? _ac_crafting))
    (return true)
    (else
      (return false))))

(fn IsGamePaused?
  (if (Math|Float|NearlyEqual(Float) (Class|GameplayStatics|GetGlobalTimeDilation) 0.0 0.01)
    (return true)
    (else
      (return false))))

(fn GetACInteraction
  (bind _returnvalue (Game|GetPlayerCharacter 0))
  (bind _returnvalue_2 (Actor|GetComponentbyClass _returnvalue "/Game/RPG_InventorySystem/Blueprints/Components/AC_Interaction.AC_Interaction_C"))
  (Utilities|IsValid _returnvalue_2
    (:Is%20Valid
      (return _returnvalue_2))))

(fn GetCurrentInteractableObject
  (bind _ac_inventory (CallFunction|GetACInventory))
  (Utilities|IsValid (Variables|/Game/RPG_InventorySystem/Blueprints/Components/AC_Inventory.AC_Inventory_C|GetCurrent%20Interactable _ac_inventory)
    (:Is%20Valid
      (return (Variables|/Game/RPG_InventorySystem/Blueprints/Components/AC_Inventory.AC_Inventory_C|GetCurrent%20Interactable _ac_inventory)))))

(fn IsValidInteractableGamepad
  (bind _ac_inventory (CallFunction|GetACInventory))
  (return (and (Utilities|IsValid (Variables|/Game/RPG_InventorySystem/Blueprints/Components/AC_Inventory.AC_Inventory_C|GetCurrent%20Interactable _ac_inventory)) (Variables|/Game/RPG_InventorySystem/Blueprints/Components/AC_Inventory.AC_Inventory_C|GetGamepadControls _ac_inventory))))

(fn AddLevelExptoPlayer
  (params (Exp%20to%20Add :type Float%20%28single-precision%29))
  (bind _returnvalue (Game|GetPlayerCharacter 0))
  (bind _returnvalue_2 (Actor|GetComponentbyClass _returnvalue "/Game/RPG_InventorySystem/Blueprints/Components/AC_Leveling.AC_Leveling_C"))
  (Utilities|IsValid _returnvalue_2
    (:Is%20Valid
      (Default|EventAddLevelExp _returnvalue_2 Exp%20to%20Add))))

(fn GetACLeveling
  (bind _returnvalue (Game|GetPlayerCharacter 0))
  (bind _returnvalue_2 (Actor|GetComponentbyClass _returnvalue "/Game/RPG_InventorySystem/Blueprints/Components/AC_Leveling.AC_Leveling_C"))
  (Utilities|IsValid _returnvalue_2
    (:Is%20Valid
      (return _returnvalue_2))))

(fn SortItemsbyType
  (params (Data%20Array :type Array%20of%20S%20Item%20Data%20Structures))
  (for _array_element Data%20Array
    (if (!= (.Class (Utilities|Struct|BreakS_ItemData _array_element)) 0)
      (Utilities|Array|Add (Utilities|Select :Index (.Type (Utilities|Struct|BreakS_ItemData _array_element)) :NewEnumerator0 0 :NewEnumerator1 (LocalVariables|GetArmor) :NewEnumerator2 (LocalVariables|GetWeapons) :NewEnumerator6 (LocalVariables|GetShields) :NewEnumerator3 (LocalVariables|GetFood) :NewEnumerator4 (LocalVariables|GetPotions) :NewEnumerator7 (LocalVariables|GetCrIngredients) :NewEnumerator8 (LocalVariables|GetQItems) :NewEnumerator5 (LocalVariables|GetOther) :NewEnumerator9 (LocalVariables|GetCurrency)) _array_element)))
  ;[0.02042 0 1 0.133] Inventory P1
  (Utilities|Array|AppendArray (LocalVariables|GetSorted) (LocalVariables|GetArmor))
  (Utilities|Array|AppendArray (LocalVariables|GetSorted) (LocalVariables|GetWeapons))
  (Utilities|Array|AppendArray (LocalVariables|GetSorted) (LocalVariables|GetShields))
  ;[0 1 0.8949 0.238] Inventory P2
  (Utilities|Array|AppendArray (LocalVariables|GetSorted) (LocalVariables|GetPotions))
  (Utilities|Array|AppendArray (LocalVariables|GetSorted) (LocalVariables|GetFood))
  ;[1 0.7568 0 0.17] Inventory P3
  (Utilities|Array|AppendArray (LocalVariables|GetSorted) (LocalVariables|GetCrIngredients))
  ;[1 0.3792 0 0.17] Inventory P4
  (Utilities|Array|AppendArray (LocalVariables|GetSorted) (LocalVariables|GetQItems))
  (Utilities|Array|AppendArray (LocalVariables|GetSorted) (LocalVariables|GetOther))
  (Utilities|Array|AppendArray (LocalVariables|GetSorted) (LocalVariables|GetCurrency))
  (return (LocalVariables|GetSorted)))

(fn SortItemsbyRarity
  (params (Data%20Array :type Array%20of%20S%20Item%20Data%20Structures))
  (for _array_element Data%20Array
    (if (!= (.Class (Utilities|Struct|BreakS_ItemData _array_element)) 0)
      (Utilities|Array|Add (Utilities|Select :Index (.Rarity (Utilities|Struct|BreakS_ItemData _array_element)) :NewEnumerator7 0 :NewEnumerator0 (LocalVariables|GetCommon) :NewEnumerator2 (LocalVariables|GetSuperior) :NewEnumerator3 (LocalVariables|GetEpic) :NewEnumerator4 (LocalVariables|GetLegendary) :NewEnumerator1 (LocalVariables|GetConsumable) :NewEnumerator5 (LocalVariables|GetUsable)) _array_element)))
  (Utilities|Array|AppendArray (LocalVariables|GetSorted) (LocalVariables|GetLegendary))
  (Utilities|Array|AppendArray (LocalVariables|GetSorted) (LocalVariables|GetEpic))
  (Utilities|Array|AppendArray (LocalVariables|GetSorted) (LocalVariables|GetSuperior))
  (Utilities|Array|AppendArray (LocalVariables|GetSorted) (LocalVariables|GetCommon))
  (Utilities|Array|AppendArray (LocalVariables|GetSorted) (LocalVariables|GetConsumable))
  (Utilities|Array|AppendArray (LocalVariables|GetSorted) (LocalVariables|GetUsable))
  (return (LocalVariables|GetSorted)))

(fn SortItemsbyValue
  (params (Data%20Array :type Array%20of%20S%20Item%20Data%20Structures))
  (for _array_element Data%20Array
    (Utilities|IsItemTypeValid? _array_element
      (:Valid
        (bind (_array_element_2 _array_index) (Utilities|Array|ForEachLoopwithBreak (LocalVariables|GetSorted) :!label _label)
          (:LoopBody
            (if (> (Utilities|Struct|BreakS_ItemStats (.Stats (Utilities|Struct|BreakS_ItemData _array_element))) (Utilities|Struct|BreakS_ItemStats (.Stats (Utilities|Struct|BreakS_ItemData _array_element_2))))
              (Utilities|FlowControl|Sequence
                (:then_0
                  (LocalVariables|SetFound true)
                  (Utilities|Array|Insert (LocalVariables|GetSorted) _array_element _array_index))
                (:then_1
                  (goto _label Break)))))
          (:Completed
            (if (LocalVariables|GetFound)
              (LocalVariables|SetFound false)
              (else
                (Utilities|Array|Add (LocalVariables|GetSorted) _array_element))))))))
  (return (LocalVariables|GetSorted)))

(fn SortItemsbyWeight
  (params (Data%20Array :type Array%20of%20S%20Item%20Data%20Structures))
  (for _array_element Data%20Array
    (if (!= (.Class (Utilities|Struct|BreakS_ItemData _array_element)) 0)
      (bind (_array_element_2 _array_index) (Utilities|Array|ForEachLoopwithBreak (LocalVariables|GetSorted) :!label _label)
        (:LoopBody
          (if (> (.Weight (Utilities|Struct|BreakS_ItemStats (.Stats (Utilities|Struct|BreakS_ItemData _array_element)))) (.Weight (Utilities|Struct|BreakS_ItemStats (.Stats (Utilities|Struct|BreakS_ItemData _array_element_2)))))
            (Utilities|FlowControl|Sequence
              (:then_0
                (LocalVariables|SetFound true)
                (Utilities|Array|Insert (LocalVariables|GetSorted) _array_element _array_index))
              (:then_1
                (goto _label Break)))))
        (:Completed
          (if (LocalVariables|GetFound)
            (LocalVariables|SetFound false)
            (else
              (Utilities|Array|Add (LocalVariables|GetSorted) _array_element)))))))
  (return (LocalVariables|GetSorted)))

(fn QuickSortItems
  (params (Data%20Array :type Array%20of%20S%20Item%20Data%20Structures))
  (for _array_element Data%20Array
    (Utilities|IsItemTypeValid? _array_element
      (:Valid
        (Utilities|Array|Add (LocalVariables|GetSorted) _array_element))))
  (return (LocalVariables|GetSorted)))

(fn GetUIBackgroundColor
  (return "(R=0.510302,G=0.515625,B=0.000000,A=1.000000)"))

(fn GetGamepadIcon
  (params (Input :type E_GamepadInputs%20Enum :default "NewEnumerator0"))
  (return (Utilities|Select :Index Input :NewEnumerator0 "/Game/RPG_InventorySystem/Textures/Images/GamepadIcons/T_Gamepad_A.T_Gamepad_A" :NewEnumerator1 "/Game/RPG_InventorySystem/Textures/Images/GamepadIcons/T_Gamepad_B.T_Gamepad_B" :NewEnumerator2 "/Game/RPG_InventorySystem/Textures/Images/GamepadIcons/T_Gamepad_X.T_Gamepad_X" :NewEnumerator3 "/Game/RPG_InventorySystem/Textures/Images/GamepadIcons/T_Gamepad_Y.T_Gamepad_Y" :NewEnumerator4 "/Game/RPG_InventorySystem/Textures/Images/GamepadIcons/T_Gamepad_LStick.T_Gamepad_LStick" :NewEnumerator5 "/Game/RPG_InventorySystem/Textures/Images/GamepadIcons/T_Gamepad_LStickDown.T_Gamepad_LStickDown" :NewEnumerator6 "/Game/RPG_InventorySystem/Textures/Images/GamepadIcons/T_Gamepad_RStick.T_Gamepad_RStick" :NewEnumerator7 "/Game/RPG_InventorySystem/Textures/Images/GamepadIcons/T_Gamepad_RStickDown.T_Gamepad_RStickDown" :NewEnumerator8 "/Game/RPG_InventorySystem/Textures/Images/GamepadIcons/T_Gamepad_LB.T_Gamepad_LB" :NewEnumerator9 "/Game/RPG_InventorySystem/Textures/Images/GamepadIcons/T_Gamepad_RB.T_Gamepad_RB" :NewEnumerator10 "/Game/RPG_InventorySystem/Textures/Images/GamepadIcons/T_Gamepad_LT.T_Gamepad_LT" :NewEnumerator11 "/Game/RPG_InventorySystem/Textures/Images/GamepadIcons/T_Gamepad_RT.T_Gamepad_RT" :NewEnumerator12 "/Game/RPG_InventorySystem/Textures/Images/GamepadIcons/T_Gamepad_DpadUp.T_Gamepad_DpadUp" :NewEnumerator13 "/Game/RPG_InventorySystem/Textures/Images/GamepadIcons/T_Gamepad_DpadDown.T_Gamepad_DpadDown" :NewEnumerator14 "/Game/RPG_InventorySystem/Textures/Images/GamepadIcons/T_Gamepad_DpadRight.T_Gamepad_DpadRight" :NewEnumerator15 "/Game/RPG_InventorySystem/Textures/Images/GamepadIcons/T_Gamepad_DpadLeft.T_Gamepad_DpadLeft" :NewEnumerator16 "/Game/RPG_InventorySystem/Textures/Images/GamepadIcons/T_Gamepad_ViewButton.T_Gamepad_ViewButton" :NewEnumerator17 "/Game/RPG_InventorySystem/Textures/Images/GamepadIcons/T_Gamepad_MenuButton.T_Gamepad_MenuButton")))

(fn PlaySoundonItemDropped
  (Audio|PlaySound2D 0 "/Game/RPG_InventorySystem/Sounds/S_Click.S_Click" 1.0 1.0 0.0 0 0))

(fn PlaySoundonOpeningWidget
  (Audio|PlaySound2D 0 "/Game/RPG_InventorySystem/Sounds/S_OpenWidget.S_OpenWidget" 1.0 1.0 0.0 0 0))

(fn PlaySoundonItemPickedUp
  (Audio|PlaySound2D 0 "/Game/RPG_InventorySystem/Sounds/S_Pickup.S_Pickup" 1.0 1.0 0.0 0 0))

(fn PlaySoundonTabSwitched
  (Audio|PlaySound2D 0 "/Game/RPG_InventorySystem/Sounds/S_Switch.S_Switch" 0.6 1.0 0.0 0 0))

(fn PlaySoundonButtonSwitched
  (Audio|PlaySound2D 0 "/Game/RPG_InventorySystem/Sounds/S_Click.S_Click" 1.0 1.0 0.0 0 0))

(fn PlaySoundonItemCrafted
  (Audio|PlaySound2D 0 "/Game/RPG_InventorySystem/Sounds/S_Craft.S_Craft" 1.0 1.0 0.0 0 0))

(fn PlaySoundonConsumableUsed
  (Audio|PlaySound2D 0 "/Game/RPG_InventorySystem/Sounds/S_Click.S_Click" 1.0 1.0 0.0 0 0))

(fn GetACActionConsumables
  (bind _returnvalue (Game|GetPlayerCharacter 0))
  (bind _returnvalue_2 (Actor|GetComponentbyClass _returnvalue "/Game/RPG_InventorySystem/Blueprints/Components/AC_ActionConsumables.AC_ActionConsumables_C"))
  (Utilities|IsValid _returnvalue_2
    (:Is%20Valid
      (return _returnvalue_2))))

(fn GetAllItemsOfType
  (params (Data%20Array :type Array%20of%20S%20Item%20Data%20Structures) (Item%20Type :type E_ItemType%20Enum :default "NewEnumerator0"))
  (for _array_element Data%20Array
    (if (Utilities|Enum|Equal(Enum) (.Type (Utilities|Struct|BreakS_ItemData _array_element)) Item%20Type)
      (Utilities|Array|Add (LocalVariables|GetItems) _array_element)))
  (return (LocalVariables|GetItems)))