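; Leveling actor component that tracks a level and experience, with thresholds loaded from a DataTable into a level-to-experience map on BeginPlay or Initialize.
; Adding experience notifies listeners, shows a notification widget and triggers LevelUp at the threshold.
; LevelUp carries surplus experience and re-triggers itself for multiple gains, clamping experience at the last defined level.
; SetLevel jumps to any valid level and resets experience to zero.
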(event Custom|Event%20Level%20Up
  ;[0 1 0.09012 0.295 22] Level UP
  (if (CallFunction|ExceedLevelMaxExp?)
    (if (CallFunction|IsNextLevelValid?)
      (Variables|Default|SetCurrent%20Experience (- (Variables|Default|GetCurrent%20Experience) (Variables|Default|GetLevel%20Max%20Experience)))
      (bind _output_get (Variables|Default|SetCurrent%20Level (+ (Variables|Default|GetCurrent%20Level) 1)))
      (Variables|Default|SetLevel%20Max%20Experience (.Value (Utilities|Map|Find (Variables|Default|GetLeveling%20Data) _output_get)))
      (Default|CallOnLevelChanged)
      (bind _returnvalue (UserInterface|CreateWidget "/Game/RPG_InventorySystem/UI/WB_LevelExpNotify.WB_LevelExpNotify_C" 0 (CallFunction|GetCurrentLevel)))
      (UserInterface|Viewport|AddtoViewport _returnvalue 0)
      (if (CallFunction|ExceedLevelMaxExp?)
        (CallFunction|EventLevelUp))
      (else
        (Variables|Default|SetCurrent%20Experience (Math|Float|Clamp(Float) (Variables|Default|GetCurrent%20Experience) 0.0 (Variables|Default|GetLevel%20Max%20Experience)))
        (Default|CallOnGainedExperience)))))

(event Custom|Event%20Add%20Level%20Exp
  (params (Experience :type Float%20%28single-precision%29))
  ;[1 0.9066 0 0.337 22] Add Level Experience
  (Variables|Default|SetCurrent%20Experience (+ Experience (Variables|Default|GetCurrent%20Experience)))
  (Default|CallOnGainedExperience)
  (bind _returnvalue (UserInterface|CreateWidget "/Game/RPG_InventorySystem/UI/WB_LevelExpNotify.WB_LevelExpNotify_C" 0 0 Experience))
  (UserInterface|Viewport|AddtoViewport _returnvalue 0)
  (if (CallFunction|ExceedLevelMaxExp?)
    (CallFunction|EventLevelUp)))

(event Custom|Event%20Set%20Level
  (params (Level :type Integer))
  (bind _leveling_data (Variables|Default|GetLeveling%20Data))
  (bind (_value _returnvalue) (Utilities|Map|Find _leveling_data Level))
  ;[0.5354 0 1 0.462] Set Current Level
  (if _returnvalue
    (Variables|Default|SetCurrent%20Level Level)
    (Variables|Default|SetLevel%20Max%20Experience _value)
    (Variables|Default|SetCurrent%20Experience 0.0)
    (Default|CallOnLevelChanged)))

(event Custom|Event%20Initialize
  (bind _leveling_data (Variables|Default|GetLeveling%20Data))
  (bind _current_level (Variables|Default|GetCurrent%20Level))
  (bind (_value _returnvalue) (Utilities|Map|Find _leveling_data _current_level))
  ;[0 0 0 0.285 22] On Begin Play - Setup Leveling Data from DataTable
  (CallFunction|SetupLevelingData)
  (if _returnvalue
    (Variables|Default|SetLevel%20Max%20Experience _value)
    (else
      (Development|PrintString "Current Level is not Valid!" true true "(R=1.000000,G=0.000000,B=0.023868,A=1.000000)" 5.0))))

(event EventBeginPlay
  (bind _leveling_data (Variables|Default|GetLeveling%20Data))
  (bind _current_level (Variables|Default|GetCurrent%20Level))
  (bind (_value _returnvalue) (Utilities|Map|Find _leveling_data _current_level))
  ;[0 0 0 0.285 22] On Begin Play - Setup Leveling Data from DataTable
  (CallFunction|SetupLevelingData)
  (if _returnvalue
    (Variables|Default|SetLevel%20Max%20Experience _value)
    (else
      (Development|PrintString "Current Level is not Valid!" true true "(R=1.000000,G=0.000000,B=0.023868,A=1.000000)" 5.0))))

(fn SetupLevelingData
  (bind _leveling_datatable (Variables|Default|GetLeveling%20DataTable))
  (bind _outrownames (DataTable|GetDataTableRowNames _leveling_datatable))
  (for _array_element _outrownames
    (bind _returnvalue (Utilities|GetDataTableRow _leveling_datatable _array_element)
      (:then
        (Utilities|Map|Add (Variables|Default|GetLeveling%20Data) (.Level (Utilities|Struct|BreakS_LevelingSystem _returnvalue)) (.Expneeded (Utilities|Struct|BreakS_LevelingSystem _returnvalue)))))))

(fn ExceedLevelMaxExp?
  (return (>= (Variables|Default|GetCurrent%20Experience) (Variables|Default|GetLevel%20Max%20Experience))))

(fn IsNextLevelValid?
  (return (.ReturnValue (Utilities|Map|Find (Variables|Default|GetLeveling%20Data) (+ (Variables|Default|GetCurrent%20Level) 1)))))

(fn GetCurrentLevel
  (return (Variables|Default|GetCurrent%20Level)))