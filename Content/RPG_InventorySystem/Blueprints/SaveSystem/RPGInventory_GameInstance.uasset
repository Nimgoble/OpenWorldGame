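; Game instance for the RPG inventory system that saves, loads, deletes and autosaves game slots.
; SaveData gathers player transform, inventory, equipment, stats, level, checkpoints, interactables and timed buffs, then writes a new numbered slot with a render-target screenshot.
; LoadData destroys checkpoints and "Destroyable" actors, respawns or restores saved state, then reinitializes inventory.
; A MetaSave indexes slot names for listing saves and loading the latest; its startup call is left unwired.
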(event Custom|Fire%20Autosave
  ;[0 1 0.1154 0.175] Autosave
  (if (Default|CanSave? (Variables|Default|GetInventory%20Component))
    (CallFunction|SaveData "NewEnumerator1")))

(event EventInit
  ;[0 0.3103 1 0.232] On Initialize Create SaveGame Object Ref. All previous saves will not appear on start  [For working in Editor]
  (bind _returnvalue (SaveGame|CreateSaveGameObject "/Game/RPG_InventorySystem/Blueprints/SaveSystem/RPGInventory_SaveGame.RPGInventory_SaveGame_C"))
  (Variables|Default|SetSaveGame _returnvalue))

(fn SaveData
  (params (Save%20Type :type E_SaveType%20Enum :default "NewEnumerator0"))
  (bind _ac_inventory (CallFunction|GetACInventory))
  (Variables|Default|SetInventory%20Component _ac_inventory)
  (bind _ac_interaction (CallFunction|GetACInteraction))
  (Variables|Default|SetInteraction%20Component _ac_interaction)
  (Utilities|FlowControl|Sequence
    (:then_0
      (Utilities|FlowControl|Sequence
        (:then_0
          (CallFunction|SaveAllCheckpoints))
        (:then_1
          (CallFunction|SavePlayerLocation))
        (:then_2
          (CallFunction|SaveAllStats))
        (:then_3
          (CallFunction|SaveInventoryandEquipment))
        (:then_4
          (CallFunction|SaveAllInteractables))
        (:then_5
          (CallFunction|SaveAllConsumableEffects))
        (:then_6
          (CallFunction|SaveLevelExperience))))
    (:then_1
      ;[1 0.02255 0 0.123] Should always be Saved as last
      (CallFunction|AssignSlotNameandData Save%20Type)
      (SaveGame|SaveGametoSlot (Variables|Default|GetSaveGame) (Variables|Default|GetSaveGameName))
      (|SaveGametoMetaSave))))

(fn LoadData
  (params (Slot%20Name :type String))
  (bind _returnvalue (SaveGame|DoesSaveGameExist Slot%20Name))
  (if _returnvalue
    (bind _returnvalue_2 (SaveGame|LoadGamefromSlot Slot%20Name))
    (bind _asrpginventory_save_game (Utilities|Casting|CastToRPGInventory_SaveGame _returnvalue_2))
    (Variables|Default|SetSaveGame _asrpginventory_save_game)
    (bind _ac_inventory (CallFunction|GetACInventory))
    (Variables|Default|SetInventory%20Component _ac_inventory)
    (bind _ac_interaction (CallFunction|GetACInteraction))
    (Variables|Default|SetInteraction%20Component _ac_interaction)
    (Utilities|FlowControl|Sequence
      (:then_0
        (Utilities|FlowControl|Sequence
          (:then_0
            (CallFunction|DestroyIndicatedActors))
          (:then_1
            (CallFunction|LoadPlayerLocation))
          (:then_2
            (CallFunction|LoadInventoryandEquipment))
          (:then_3
            (CallFunction|LoadAllInteractables))
          (:then_4
            (CallFunction|LoadAllCheckpoints))
          (:then_5
            (CallFunction|LoadAllConsumableEffects))
          (:then_6
            (CallFunction|LoadAllStats))
          (:then_7
            (CallFunction|LoadLevelExperience))))
      (:then_1
        ;[1 0 0 0.238] Re-initalize Inventory at the end
        (Default|InitializeInventory (Variables|Default|GetInventory%20Component))
        (Default|RemoveInventoryWidget (Variables|Default|GetInventory%20Component))
        (Default|RefreshEquipment (Variables|Default|GetInventory%20Component))))))

(fn SavePlayerLocation
  (Variables|/Game/RPG_InventorySystem/Blueprints/SaveSystem/RPGInventory_SaveGame.RPGInventory_SaveGame_C|SetPlayer%20Transform (Variables|Default|GetSaveGame) (Transformation|GetActorTransform (Variables|/Game/RPG_InventorySystem/Blueprints/Components/AC_Inventory.AC_Inventory_C|GetPlayer%20Ref (Variables|Default|GetInventory%20Component)))))

(fn SaveInventoryandEquipment
  (bind _inventory_component (Variables|Default|GetInventory%20Component))
  (Variables|/Game/RPG_InventorySystem/Blueprints/SaveSystem/RPGInventory_SaveGame.RPGInventory_SaveGame_C|SetInventoryP1 (Variables|Default|GetSaveGame) (Variables|/Game/RPG_InventorySystem/Blueprints/Components/AC_Inventory.AC_Inventory_C|GetInventory%20P1 _inventory_component))
  (Variables|/Game/RPG_InventorySystem/Blueprints/SaveSystem/RPGInventory_SaveGame.RPGInventory_SaveGame_C|SetInventoryP2 (Variables|Default|GetSaveGame) (Variables|/Game/RPG_InventorySystem/Blueprints/Components/AC_Inventory.AC_Inventory_C|GetInventory%20P2 _inventory_component))
  (Variables|/Game/RPG_InventorySystem/Blueprints/SaveSystem/RPGInventory_SaveGame.RPGInventory_SaveGame_C|SetInventoryP3 (Variables|Default|GetSaveGame) (Variables|/Game/RPG_InventorySystem/Blueprints/Components/AC_Inventory.AC_Inventory_C|GetInventory%20P3 _inventory_component))
  (Variables|/Game/RPG_InventorySystem/Blueprints/SaveSystem/RPGInventory_SaveGame.RPGInventory_SaveGame_C|SetInventoryP4 (Variables|Default|GetSaveGame) (Variables|/Game/RPG_InventorySystem/Blueprints/Components/AC_Inventory.AC_Inventory_C|GetInventory%20P4 _inventory_component))
  (Variables|/Game/RPG_InventorySystem/Blueprints/SaveSystem/RPGInventory_SaveGame.RPGInventory_SaveGame_C|SetEquipment (Variables|Default|GetSaveGame) (Variables|/Game/RPG_InventorySystem/Blueprints/Components/AC_Inventory.AC_Inventory_C|GetEquipment%20Data _inventory_component)))

(fn LoadPlayerLocation
  (bind _inventory_component (Variables|Default|GetInventory%20Component))
  (bind _player_ref (Variables|/Game/RPG_InventorySystem/Blueprints/Components/AC_Inventory.AC_Inventory_C|GetPlayer%20Ref _inventory_component))
  (bind _charactermovement (Variables|/Script/Engine.Character|GetCharacterMovement _player_ref))
  (Transformation|SetActorTransform _player_ref (Variables|/Game/RPG_InventorySystem/Blueprints/SaveSystem/RPGInventory_SaveGame.RPGInventory_SaveGame_C|GetPlayer%20Transform (Variables|Default|GetSaveGame)))
  (Pawn|Components|CharacterMovement|DisableMovement _charactermovement)
  (Pawn|Components|CharacterMovement|SetMovementMode _charactermovement "MOVE_Walking" 0))

(fn LoadInventoryandEquipment
  (bind _inventory_component (Variables|Default|GetInventory%20Component))
  (bind _inventory_component_2 (Variables|Default|GetInventory%20Component))
  ;[1 0 0.02652 0.352] Detach Current Equipment
  (bind _enumvalue (|ForEachE_ItemSlot)
    (:LoopBody
      (bind _structout (Utilities|Struct|SetmembersinS_ItemData (LocalVariables|GetL%20Empty%20Data) _enumvalue))
      (Default|DetachItemfromEquipment _inventory_component _structout)
      (Default|EventDetachfromPlayerCapture (Variables|/Game/RPG_InventorySystem/Blueprints/Components/AC_Inventory.AC_Inventory_C|GetCapture%20Ref _inventory_component) _structout))
    (:then
      ;[0.1673 1 0.027 0.196] Attach Equipment from Save
      (bind _enumvalue_2 (|ForEachE_ItemSlot)
        (:LoopBody
          (if (.ReturnValue (Utilities|Map|Find (Variables|/Game/RPG_InventorySystem/Blueprints/SaveSystem/RPGInventory_SaveGame.RPGInventory_SaveGame_C|GetEquipment (Variables|Default|GetSaveGame)) _enumvalue_2))
            (Default|AttachItemtoEquipment _inventory_component_2 (.Value (Utilities|Map|Find (Variables|/Game/RPG_InventorySystem/Blueprints/SaveSystem/RPGInventory_SaveGame.RPGInventory_SaveGame_C|GetEquipment (Variables|Default|GetSaveGame)) _enumvalue_2)))
            (Default|EventAttachtoPlayerCapture (Variables|/Game/RPG_InventorySystem/Blueprints/Components/AC_Inventory.AC_Inventory_C|GetCapture%20Ref _inventory_component_2) (.Value (Utilities|Map|Find (Variables|/Game/RPG_InventorySystem/Blueprints/SaveSystem/RPGInventory_SaveGame.RPGInventory_SaveGame_C|GetEquipment (Variables|Default|GetSaveGame)) _enumvalue_2)))))
        (:then
          (Utilities|FlowControl|Sequence
            (:then_0
              (Variables|/Game/RPG_InventorySystem/Blueprints/Components/AC_Inventory.AC_Inventory_C|SetInventory%20P1 (Variables|Default|GetInventory%20Component) (Variables|/Game/RPG_InventorySystem/Blueprints/SaveSystem/RPGInventory_SaveGame.RPGInventory_SaveGame_C|GetInventoryP1 (Variables|Default|GetSaveGame))))
            (:then_1
              (Variables|/Game/RPG_InventorySystem/Blueprints/Components/AC_Inventory.AC_Inventory_C|SetInventory%20P2 (Variables|Default|GetInventory%20Component) (Variables|/Game/RPG_InventorySystem/Blueprints/SaveSystem/RPGInventory_SaveGame.RPGInventory_SaveGame_C|GetInventoryP2 (Variables|Default|GetSaveGame))))
            (:then_2
              (Variables|/Game/RPG_InventorySystem/Blueprints/Components/AC_Inventory.AC_Inventory_C|SetInventory%20P3 (Variables|Default|GetInventory%20Component) (Variables|/Game/RPG_InventorySystem/Blueprints/SaveSystem/RPGInventory_SaveGame.RPGInventory_SaveGame_C|GetInventoryP3 (Variables|Default|GetSaveGame))))
            (:then_3
              (Variables|/Game/RPG_InventorySystem/Blueprints/Components/AC_Inventory.AC_Inventory_C|SetInventory%20P4 (Variables|Default|GetInventory%20Component) (Variables|/Game/RPG_InventorySystem/Blueprints/SaveSystem/RPGInventory_SaveGame.RPGInventory_SaveGame_C|GetInventoryP4 (Variables|Default|GetSaveGame))))
            (:then_4
              (Variables|/Game/RPG_InventorySystem/Blueprints/Components/AC_Inventory.AC_Inventory_C|SetEquipment%20Data (Variables|Default|GetInventory%20Component) (Variables|/Game/RPG_InventorySystem/Blueprints/SaveSystem/RPGInventory_SaveGame.RPGInventory_SaveGame_C|GetEquipment (Variables|Default|GetSaveGame))))))))))

(fn SaveAllStats
  (bind _inventory_component (Variables|Default|GetInventory%20Component))
  (Utilities|Struct|SetmembersinS_SaveStats (Variables|/Game/RPG_InventorySystem/Blueprints/SaveSystem/RPGInventory_SaveGame.RPGInventory_SaveGame_C|GetStats (Variables|Default|GetSaveGame)) (Variables|/Game/RPG_InventorySystem/Blueprints/Components/AC_Inventory.AC_Inventory_C|GetPlayer%20Gold _inventory_component) (Variables|/Game/RPG_InventorySystem/Blueprints/Components/AC_Inventory.AC_Inventory_C|GetCurrent%20Inventory%20Weight _inventory_component) (Variables|/Game/RPG_InventorySystem/Blueprints/Components/AC_Inventory.AC_Inventory_C|GetMax%20Inventory%20Weight _inventory_component) (Variables|/Game/RPG_InventorySystem/Blueprints/Components/AC_Inventory.AC_Inventory_C|GetStats _inventory_component)))

(fn LoadAllStats
  (bind _savegame (Variables|Default|GetSaveGame))
  (bind _stats (Variables|/Game/RPG_InventorySystem/Blueprints/SaveSystem/RPGInventory_SaveGame.RPGInventory_SaveGame_C|GetStats _savegame))
  (bind (_gold _currentinventoryweight _maxinventoryweight _stats_2) (Utilities|Struct|BreakS_SaveStats _stats))
  (Utilities|FlowControl|Sequence
    (:then_0
      (Variables|/Game/RPG_InventorySystem/Blueprints/Components/AC_Inventory.AC_Inventory_C|SetPlayer%20Gold (Variables|Default|GetInventory%20Component) _gold)
      (Variables|/Game/RPG_InventorySystem/Blueprints/Components/AC_Inventory.AC_Inventory_C|SetCurrent%20Inventory%20Weight (Variables|Default|GetInventory%20Component) _currentinventoryweight)
      (Variables|/Game/RPG_InventorySystem/Blueprints/Components/AC_Inventory.AC_Inventory_C|SetMax%20Inventory%20Weight (Variables|Default|GetInventory%20Component) _maxinventoryweight)
      (for _array_element _stats_2
        (Default|SetStatValue (Variables|Default|GetInventory%20Component) (.stat _array_element) (.value _array_element))))))

(fn LoadAllInteractables
  (for _array_element (Variables|/Game/RPG_InventorySystem/Blueprints/SaveSystem/RPGInventory_SaveGame.RPGInventory_SaveGame_C|GetInteractables (Variables|Default|GetSaveGame))
    (bind _output_get (LocalVariables|SetL%20Saved%20Interactable%20Data _array_element))
    (if (.DestroyAfterPickup (Utilities|Struct|BreakS_SaveInteractables _output_get))
      (bind _returnvalue (Game|SpawnActorfromClass (.SpawnActorClass (Utilities|Struct|BreakS_SaveInteractables _output_get)) (.Transform (Utilities|Struct|BreakS_SaveInteractables _output_get)) "AlwaysSpawn" 0 0))
      (LocalVariables|SetL%20Spawned%20Interactable _returnvalue)
      (else
        (bind _output_get_2 (LocalVariables|SetL%20Spawned%20Interactable (.InteractableActor (Utilities|Struct|BreakS_SaveInteractables _output_get))))
        (Transformation|SetActorTransform _output_get_2 (.Transform (Utilities|Struct|BreakS_SaveInteractables _output_get)))))
    (Utilities|IsValid (Actor|GetComponentbyClass (LocalVariables|GetL%20Spawned%20Interactable) "/Game/RPG_InventorySystem/Blueprints/Components/AC_Interactable.AC_Interactable_C")
      (:Is%20Valid
        (LocalVariables|SetL%20Interactable%20Component (Actor|GetComponentbyClass (LocalVariables|GetL%20Spawned%20Interactable) "/Game/RPG_InventorySystem/Blueprints/Components/AC_Interactable.AC_Interactable_C"))
        ;[1 0.0344 0 0.138] Re-initialize Interaction
        (Default|RemoveInteractionfromCurrent (Variables|Default|GetInteraction%20Component))
        (Default|EventInitialize (LocalVariables|GetL%20Interactable%20Component))
        (Variables|/Game/RPG_InventorySystem/Blueprints/Components/AC_Interactable.AC_Interactable_C|SetItemData (LocalVariables|GetL%20Interactable%20Component) (.itemdata (LocalVariables|GetL%20Saved%20Interactable%20Data)))
        (Variables|/Game/RPG_InventorySystem/Blueprints/Components/AC_Interactable.AC_Interactable_C|SetDestroy%20after%20Pickup? (LocalVariables|GetL%20Interactable%20Component) (.destroyafterpickup (LocalVariables|GetL%20Saved%20Interactable%20Data)))
        (Variables|/Game/RPG_InventorySystem/Blueprints/Components/AC_Interactable.AC_Interactable_C|SetInventory%20Size%28Vendor/Storage%29 (LocalVariables|GetL%20Interactable%20Component) (.inventorysize (LocalVariables|GetL%20Saved%20Interactable%20Data)))
        (Variables|/Game/RPG_InventorySystem/Blueprints/Components/AC_Interactable.AC_Interactable_C|SetVendor%20Gold (LocalVariables|GetL%20Interactable%20Component) (.vendorgold (LocalVariables|GetL%20Saved%20Interactable%20Data)))
        (Utilities|IsValid (.attachedparentactor (LocalVariables|GetL%20Saved%20Interactable%20Data))
          (:Is%20Valid
            (Transformation|AttachActorToActor (LocalVariables|GetL%20Spawned%20Interactable) (.attachedparentactor (LocalVariables|GetL%20Saved%20Interactable%20Data)) "None" "KeepWorld" "KeepWorld" "KeepWorld" true))
          (:Is%20Not%20Valid
            _))
        (Variables|/Game/RPG_InventorySystem/Blueprints/Components/AC_Interactable.AC_Interactable_C|SetIsInteractable (LocalVariables|GetL%20Interactable%20Component) (.isinteractable (LocalVariables|GetL%20Saved%20Interactable%20Data)))
        (Variables|/Game/RPG_InventorySystem/Blueprints/Components/AC_Interactable.AC_Interactable_C|SetInteractable%20Response (LocalVariables|GetL%20Interactable%20Component) (.interactionresponse (LocalVariables|GetL%20Saved%20Interactable%20Data)))
        (Variables|/Game/RPG_InventorySystem/Blueprints/Components/AC_Interactable.AC_Interactable_C|SetInteractable%20Value (LocalVariables|GetL%20Interactable%20Component) (.interactionvalue (LocalVariables|GetL%20Saved%20Interactable%20Data)))
        (Variables|/Game/RPG_InventorySystem/Blueprints/Components/AC_Interactable.AC_Interactable_C|SetAlready%20Interacted (LocalVariables|GetL%20Interactable%20Component) (.alreadyinteracted (LocalVariables|GetL%20Saved%20Interactable%20Data)))
        (Variables|/Game/RPG_InventorySystem/Blueprints/Components/AC_Interactable.AC_Interactable_C|SetTimeline%20Direction (LocalVariables|GetL%20Interactable%20Component) (.timelinedirection (LocalVariables|GetL%20Saved%20Interactable%20Data)))
        (Variables|/Game/RPG_InventorySystem/Blueprints/Components/AC_Interactable.AC_Interactable_C|SetTimeline%20Position (LocalVariables|GetL%20Interactable%20Component) (.timelinepostion (LocalVariables|GetL%20Saved%20Interactable%20Data)))
        ;[0.5601 0 1 0.211] Call Event GameLoaded for Interactables
        (Default|EventGameLoaded (LocalVariables|GetL%20Interactable%20Component))))))

(fn SaveAllInteractables
  (bind _outactors (Actor|GetAllActorswithTag "Interactable"))
  (for _array_element _outactors
    (Utilities|IsValid (Actor|GetComponentbyClass _array_element "/Game/RPG_InventorySystem/Blueprints/Components/AC_Interactable.AC_Interactable_C")
      (:Is%20Valid
        (LocalVariables|SetL%20Interactable%20Component (Actor|GetComponentbyClass _array_element "/Game/RPG_InventorySystem/Blueprints/Components/AC_Interactable.AC_Interactable_C"))
        (Utilities|Array|Add (LocalVariables|GetInteractables) (Utilities|Struct|MakeS_SaveInteractables _array_element (Utilities|GetClass _array_element) (Transformation|GetActorTransform _array_element) (Variables|/Game/RPG_InventorySystem/Blueprints/Components/AC_Interactable.AC_Interactable_C|GetItemData (LocalVariables|GetL%20Interactable%20Component)) (Variables|/Game/RPG_InventorySystem/Blueprints/Components/AC_Interactable.AC_Interactable_C|GetDestroy%20after%20Pickup? (LocalVariables|GetL%20Interactable%20Component)) (Variables|/Game/RPG_InventorySystem/Blueprints/Components/AC_Interactable.AC_Interactable_C|GetInventory%20Size%28Vendor/Storage%29 (LocalVariables|GetL%20Interactable%20Component)) (Variables|/Game/RPG_InventorySystem/Blueprints/Components/AC_Interactable.AC_Interactable_C|GetVendor%20Gold (LocalVariables|GetL%20Interactable%20Component)) (Variables|/Game/RPG_InventorySystem/Blueprints/Components/AC_Interactable.AC_Interactable_C|GetIsInteractable (LocalVariables|GetL%20Interactable%20Component)) (select (Utilities|IsValid (Actor|GetAttachParentActor _array_element)) (Actor|GetAttachParentActor _array_element) 0) (Variables|/Game/RPG_InventorySystem/Blueprints/Components/AC_Interactable.AC_Interactable_C|GetTimeline%20Position (LocalVariables|GetL%20Interactable%20Component)) (Variables|/Game/RPG_InventorySystem/Blueprints/Components/AC_Interactable.AC_Interactable_C|GetTimeline%20Direction (LocalVariables|GetL%20Interactable%20Component)) (Variables|/Game/RPG_InventorySystem/Blueprints/Components/AC_Interactable.AC_Interactable_C|GetAlready%20Interacted (LocalVariables|GetL%20Interactable%20Component)) (Variables|/Game/RPG_InventorySystem/Blueprints/Components/AC_Interactable.AC_Interactable_C|GetInteractable%20Value (LocalVariables|GetL%20Interactable%20Component)) (Variables|/Game/RPG_InventorySystem/Blueprints/Components/AC_Interactable.AC_Interactable_C|GetInteractable%20Response (LocalVariables|GetL%20Interactable%20Component)))))))
  (Variables|/Game/RPG_InventorySystem/Blueprints/SaveSystem/RPGInventory_SaveGame.RPGInventory_SaveGame_C|SetInteractables (Variables|Default|GetSaveGame) (LocalVariables|GetInteractables)))

(fn DeleteData
  (params (SlotName :type String))
  (bind _metasave (Variables|Default|GetMetaSave))
  (SaveGame|DeleteGameinSlot SlotName)
  (Utilities|IsValid _metasave
    (:Is%20Valid
      (Utilities|Array|RemoveItem (Variables|/Game/RPG_InventorySystem/Blueprints/SaveSystem/Meta_SaveGame.Meta_SaveGame_C|GetSlotNames _metasave) SlotName)
      (SaveGame|SaveGametoSlot (Variables|Default|GetMetaSave) "MetaSave"))))

(fn Autosave
  (params (Type :type E_AutosaveTimer%20Enum :default "NewEnumerator4"))
  (bind _output_get (Variables|Default|SetAutosaveFrequency Type))
  (if (Utilities|Enum|NotEqual(Enum) _output_get "NewEnumerator4")
    (bind _returnvalue (Utilities|Time|SetTimerbyEvent (EventDispatchers|CreateEvent :!event Custom|Fire%20Autosave) (Utilities|Select :Index _output_get :NewEnumerator4 0.0 :NewEnumerator2 6e+02 :NewEnumerator1 3e+02 :NewEnumerator3 1.8e+02 :NewEnumerator0 6e+01) true))
    (LocalVariables|SetAutosaveTimer _returnvalue)
    (else
      (Utilities|Time|PauseTimerbyHandle (LocalVariables|GetAutosaveTimer)))))

(fn AssignSlotNameandData
  (params (SaveType :type E_SaveType%20Enum :default "NewEnumerator0"))
  (bind _returnvalue (Class|KismetSystemLibrary|GetProjectSavedDirectory))
  (bind _slotsuffix (Variables|Default|GetSlotSuffix))
  (bind _returnvalue_2 (Utilities|String|Append _returnvalue "SaveGames/"))
  (Math|Integer|IncrementInt _slotsuffix
    (:%20%20
      (Variables|Default|SetSaveGameName (Utilities|String|Append (Utilities|String|EnumtoString SaveType) "_" "Slot" (Utilities|String|ToString(Integer) _slotsuffix)))
      (Rendering|SceneCapture|CaptureScene (Variables|/Game/RPG_InventorySystem/ThirdPersonExample/Blueprints/BP_RPGInventoryCharacter.BP_RPGInventoryCharacter_C|GetSaveGameCapture (Variables|/Game/RPG_InventorySystem/Blueprints/Components/AC_Inventory.AC_Inventory_C|GetPlayer%20Ref (Variables|Default|GetInventory%20Component))) :!class /Script/Engine.SceneCaptureComponent2D)
      (Rendering|ExportRenderTarget "/Game/RPG_InventorySystem/Blueprints/SaveSystem/RT_SaveGameCapture.RT_SaveGameCapture" _returnvalue_2 (Utilities|String|Append (Variables|Default|GetSaveGameName) ".png"))
      (Utilities|Array|Add (Variables|Default|GetSaveSlots) (Utilities|Struct|MakeS_SaveSlotDetails (Variables|Default|GetSaveGameName) (Math|DateTime|UTCNow) SaveType 0 (Utilities|String|Append _returnvalue_2 (Utilities|String|Append (Variables|Default|GetSaveGameName) ".png"))))
      (Variables|/Game/RPG_InventorySystem/Blueprints/SaveSystem/RPGInventory_SaveGame.RPGInventory_SaveGame_C|SetSaveSlot (Variables|Default|GetSaveGame) (Utilities|Struct|MakeS_SaveSlotDetails (Variables|Default|GetSaveGameName) (Math|DateTime|UTCNow) SaveType 0 (Utilities|String|Append _returnvalue_2 (Utilities|String|Append (Variables|Default|GetSaveGameName) ".png")))))))

(fn SaveAllCheckpoints
  (bind _outactors (Actor|GetAllActorsOfClass "/Game/RPG_InventorySystem/Blueprints/SaveSystem/BP_CheckpointSave.BP_CheckpointSave_C"))
  (for _array_element _outactors
    (Utilities|Array|Add (LocalVariables|GetCheckpoints) (Utilities|Struct|MakeS_SaveCheckpoints (Utilities|GetClass _array_element) (Transformation|GetActorTransform _array_element))))
  (Variables|/Game/RPG_InventorySystem/Blueprints/SaveSystem/RPGInventory_SaveGame.RPGInventory_SaveGame_C|SetCheckpoints (Variables|Default|GetSaveGame) (LocalVariables|GetCheckpoints)))

(fn LoadAllCheckpoints
  (for _array_element (Variables|/Game/RPG_InventorySystem/Blueprints/SaveSystem/RPGInventory_SaveGame.RPGInventory_SaveGame_C|GetCheckpoints (Variables|Default|GetSaveGame))
    (Game|SpawnActorfromClass (.checkpoint _array_element) (.transform _array_element) "Undefined" 0 0)))

(fn SaveAllConsumableEffects
  (for _array_element (CallFunction|GetAllConsumableData)
    (if (!= (Utilities|Struct|BreakS_ConsumableAction (Utilities|Struct|BreakS_SaveBuffs _array_element)) 0.0)
      (bind _structout (Utilities|Struct|SetmembersinS_SaveBuffs _array_element (/ 1.0 (Utilities|Struct|BreakS_ConsumableAction (Utilities|Struct|BreakS_SaveBuffs _array_element)))))
      (switch Utilities|FlowControl|Switch|SwitchonE_EffectCategory (.Category (Utilities|Struct|BreakS_ConsumableAction (.BuffData (Utilities|Struct|BreakS_SaveBuffs _structout))))
        (:NewEnumerator2
          (Utilities|Array|Add (LocalVariables|GetConsumables) (Utilities|Struct|MakeS_SaveBuffs (.BuffData (Utilities|Struct|BreakS_SaveBuffs _structout)) (.CurrentReps (Utilities|Struct|BreakS_SaveBuffs _structout)) (.TimerHandle (Utilities|Struct|BreakS_SaveBuffs _structout)) (Components|Timeline|GetPlaybackPosition (CallFunction|GetTimelineBaseonStat (.Stat (Utilities|Struct|BreakS_ConsumableAction (.BuffData (Utilities|Struct|BreakS_SaveBuffs _structout)))))) (.PlayRate (Utilities|Struct|BreakS_SaveBuffs _structout)))))
        (:NewEnumerator3
          (bind _structout_2 (Utilities|Struct|SetmembersinS_ConsumableAction (.BuffData (Utilities|Struct|BreakS_SaveBuffs _structout)) (Utilities|Time|GetTimerRemainingTimebyHandle (.TimerHandle (Utilities|Struct|BreakS_SaveBuffs _structout)))))
          (Utilities|Array|Add (LocalVariables|GetConsumables) (Utilities|Struct|MakeS_SaveBuffs _structout_2 (.CurrentReps (Utilities|Struct|BreakS_SaveBuffs _structout)) (.TimerHandle (Utilities|Struct|BreakS_SaveBuffs _structout)) (Components|Timeline|GetPlaybackPosition (CallFunction|GetTimelineBaseonStat (.Stat (Utilities|Struct|BreakS_ConsumableAction (.BuffData (Utilities|Struct|BreakS_SaveBuffs _structout)))))) (.PlayRate (Utilities|Struct|BreakS_SaveBuffs _structout))))))))
  (Variables|/Game/RPG_InventorySystem/Blueprints/SaveSystem/RPGInventory_SaveGame.RPGInventory_SaveGame_C|SetCurrentBuffs (Variables|Default|GetSaveGame) (LocalVariables|GetConsumables)))

(fn LoadAllConsumableEffects
  (bind _inventory_component (Variables|Default|GetInventory%20Component))
  (bind _inventory_component_2 (Variables|Default|GetInventory%20Component))
  (bind _capture_ref (Variables|/Game/RPG_InventorySystem/Blueprints/Components/AC_Inventory.AC_Inventory_C|GetCapture%20Ref _inventory_component))
  (bind _action_consumables_component (Variables|/Game/RPG_InventorySystem/Blueprints/Components/AC_Inventory.AC_Inventory_C|GetAction%20Consumables%20Component _inventory_component_2))
  (bind _returnvalue (CallFunction|GetACActionConsumables))
  (LocalVariables|SetL%20Action%20Consumables _returnvalue)
  ;[1 0.1477 0 0.133] Clear Current Effects and Timers
  (for _array_element (CallFunction|GetAllConsumableData)
    (Utilities|Time|PauseTimerbyHandle (.timerhandle _array_element))
    (Default|RemoveAdditionalEffect (Variables|/Game/RPG_InventorySystem/Blueprints/Components/AC_Inventory.AC_Inventory_C|GetCapture%20Ref (Variables|Default|GetInventory%20Component)) (.AdditionalEffects (Utilities|Struct|BreakS_ConsumableAction (.buffdata _array_element))))
    (Utilities|IsValid (CallFunction|GetTimelineBaseonStat (.Stat (Utilities|Struct|BreakS_ConsumableAction (.buffdata _array_element))))
      (:Is%20Valid
        (Components|Timeline|SetPlaybackPosition (CallFunction|GetTimelineBaseonStat (.Stat (Utilities|Struct|BreakS_ConsumableAction (.buffdata _array_element)))) 1.0 false true)
        (Default|EventInitializeCircularAnimation (LocalVariables|GetL%20Action%20Consumables) (.Stat (Utilities|Struct|BreakS_ConsumableAction (.buffdata _array_element))))
        (switch Utilities|FlowControl|Switch|SwitchonE_EffectCategory (.Category (Utilities|Struct|BreakS_ConsumableAction (.buffdata _array_element)))
          (:NewEnumerator3
            (switch Utilities|FlowControl|Switch|SwitchonE_StatCategory (Utilities|Struct|BreakS_ConsumableAction (.buffdata _array_element))
              (:NewEnumerator6
                (Default|ClearMaxHealthFD (LocalVariables|GetL%20Action%20Consumables)))
              (:NewEnumerator7
                (Default|ClearMaxStaminaFD (LocalVariables|GetL%20Action%20Consumables)))
              (:NewEnumerator2
                (Default|ClearArmorFD (LocalVariables|GetL%20Action%20Consumables)))
              (:NewEnumerator3
                (Default|ClearDamageFD (LocalVariables|GetL%20Action%20Consumables)))
              (:NewEnumerator4
                (Default|ClearAttackSpeedFD (LocalVariables|GetL%20Action%20Consumables)))))))))
  (for _array_element_2 (Variables|/Game/RPG_InventorySystem/Blueprints/SaveSystem/RPGInventory_SaveGame.RPGInventory_SaveGame_C|GetCurrentBuffs (Variables|Default|GetSaveGame))
    (switch Utilities|FlowControl|Switch|SwitchonE_EffectCategory (Utilities|Struct|BreakS_ConsumableAction (Utilities|Struct|BreakS_SaveBuffs _array_element_2))
      (:NewEnumerator2
        (Default|AddOverDurationfromSave _action_consumables_component _array_element_2))
      (:NewEnumerator3
        (Default|AddforDurationfromSave _action_consumables_component _array_element_2)))
    (Default|EventInitializeCircularAnimation (LocalVariables|GetL%20Action%20Consumables) (.Stat (Utilities|Struct|BreakS_ConsumableAction (.BuffData (Utilities|Struct|BreakS_SaveBuffs _array_element_2)))))
    (Components|Timeline|SetPlaybackPosition (CallFunction|GetTimelineBaseonStat (.Stat (Utilities|Struct|BreakS_ConsumableAction (.BuffData (Utilities|Struct|BreakS_SaveBuffs _array_element_2))))) (.TimelinePosition (Utilities|Struct|BreakS_SaveBuffs _array_element_2)) false true)
    (Components|Timeline|SetPlayRate (CallFunction|GetTimelineBaseonStat (.Stat (Utilities|Struct|BreakS_ConsumableAction (.BuffData (Utilities|Struct|BreakS_SaveBuffs _array_element_2))))) (.PlayRate (Utilities|Struct|BreakS_SaveBuffs _array_element_2)))
    (Default|PlayTimeline _capture_ref)
    (Default|AssignAdditionalEffect _capture_ref (.Stat (Utilities|Struct|BreakS_ConsumableAction (.BuffData (Utilities|Struct|BreakS_SaveBuffs _array_element_2)))) (.AdditionalEffects (Utilities|Struct|BreakS_ConsumableAction (.BuffData (Utilities|Struct|BreakS_SaveBuffs _array_element_2)))))
    (Default|PlayAdditionalEffect _capture_ref (.AdditionalEffects (Utilities|Struct|BreakS_ConsumableAction (.BuffData (Utilities|Struct|BreakS_SaveBuffs _array_element_2)))))))

(fn GetTimelineBaseonStat
  (params (Stat :type E_StatCategory%20Enum :default "NewEnumerator8"))
  (bind _inventory_component (Variables|Default|GetInventory%20Component))
  (bind _capture_ref (Variables|/Game/RPG_InventorySystem/Blueprints/Components/AC_Inventory.AC_Inventory_C|GetCapture%20Ref _inventory_component))
  (return (Utilities|Select :Index Stat :NewEnumerator8 0 :NewEnumerator0 (Variables|/Game/RPG_InventorySystem/Blueprints/Capture/BP_PlayerCapture.BP_PlayerCapture_C|GetHealthTimeline _capture_ref) :NewEnumerator6 (Variables|/Game/RPG_InventorySystem/Blueprints/Capture/BP_PlayerCapture.BP_PlayerCapture_C|GetMaxHealthTimeline _capture_ref) :NewEnumerator1 (Variables|/Game/RPG_InventorySystem/Blueprints/Capture/BP_PlayerCapture.BP_PlayerCapture_C|GetStaminaTimeline _capture_ref) :NewEnumerator7 (Variables|/Game/RPG_InventorySystem/Blueprints/Capture/BP_PlayerCapture.BP_PlayerCapture_C|GetMaxStaminaTimeline _capture_ref) :NewEnumerator2 (Variables|/Game/RPG_InventorySystem/Blueprints/Capture/BP_PlayerCapture.BP_PlayerCapture_C|GetArmorTimeline _capture_ref) :NewEnumerator3 (Variables|/Game/RPG_InventorySystem/Blueprints/Capture/BP_PlayerCapture.BP_PlayerCapture_C|GetDamageTimeline _capture_ref) :NewEnumerator4 (Variables|/Game/RPG_InventorySystem/Blueprints/Capture/BP_PlayerCapture.BP_PlayerCapture_C|GetAttackSpeedTimeline _capture_ref))))

(fn GetAllConsumableData
  (bind _inventory_component (Variables|Default|GetInventory%20Component))
  (bind _action_consumables_component (Variables|/Game/RPG_InventorySystem/Blueprints/Components/AC_Inventory.AC_Inventory_C|GetAction%20Consumables%20Component _inventory_component))
  (return (Utilities|Array|MakeArray (Variables|/Game/RPG_InventorySystem/Blueprints/Components/AC_ActionConsumables.AC_ActionConsumables_C|GetHealthEffectData _action_consumables_component) (Variables|/Game/RPG_InventorySystem/Blueprints/Components/AC_ActionConsumables.AC_ActionConsumables_C|GetMaxHealthEffectData _action_consumables_component) (Variables|/Game/RPG_InventorySystem/Blueprints/Components/AC_ActionConsumables.AC_ActionConsumables_C|GetStaminaEffectData _action_consumables_component) (Variables|/Game/RPG_InventorySystem/Blueprints/Components/AC_ActionConsumables.AC_ActionConsumables_C|GetMaxStaminaEffectData _action_consumables_component) (Variables|/Game/RPG_InventorySystem/Blueprints/Components/AC_ActionConsumables.AC_ActionConsumables_C|GetArmorEffectData _action_consumables_component) (Variables|/Game/RPG_InventorySystem/Blueprints/Components/AC_ActionConsumables.AC_ActionConsumables_C|GetDamageEffectData _action_consumables_component) (Variables|/Game/RPG_InventorySystem/Blueprints/Components/AC_ActionConsumables.AC_ActionConsumables_C|GetAttackSpeedEffectData _action_consumables_component))))

(fn DestroyIndicatedActors
  ;[1 0.1289 0] Destroy Checkpoints
  (bind _outactors (Actor|GetAllActorsOfClass "/Game/RPG_InventorySystem/Blueprints/SaveSystem/BP_CheckpointSave.BP_CheckpointSave_C"))
  (for _array_element _outactors
    (Actor|DestroyActor _array_element))
  (bind _outactors_2 (Actor|GetAllActorswithTag "Destroyable"))
  (for _array_element_2 _outactors_2
    (Actor|DestroyActor _array_element_2)))

(fn SaveLevelExperience
  (bind _return_value (CallFunction|GetACLeveling))
  (Utilities|Struct|SetmembersinS_LevelingSystem (Variables|/Game/RPG_InventorySystem/Blueprints/SaveSystem/RPGInventory_SaveGame.RPGInventory_SaveGame_C|GetLevel%20Exp (Variables|Default|GetSaveGame)) (Variables|/Game/RPG_InventorySystem/Blueprints/Components/AC_Leveling.AC_Leveling_C|GetCurrent%20Level _return_value) (Variables|/Game/RPG_InventorySystem/Blueprints/Components/AC_Leveling.AC_Leveling_C|GetCurrent%20Experience _return_value)))

(fn LoadLevelExperience
  (bind _savegame (Variables|Default|GetSaveGame))
  (bind _level_exp (Variables|/Game/RPG_InventorySystem/Blueprints/SaveSystem/RPGInventory_SaveGame.RPGInventory_SaveGame_C|GetLevel%20Exp _savegame))
  (bind _return_value (CallFunction|GetACLeveling))
  (Variables|/Game/RPG_InventorySystem/Blueprints/Components/AC_Leveling.AC_Leveling_C|SetCurrent%20Level _return_value (.level _level_exp))
  (Variables|/Game/RPG_InventorySystem/Blueprints/Components/AC_Leveling.AC_Leveling_C|SetCurrent%20Experience _return_value (.expneeded _level_exp))
  (Default|EventInitialize _return_value))

(event Custom|Load%20Most%20Recent%20Save
  (bind _metasave (Variables|Default|GetMetaSave))
  (bind _slotnames (Variables|/Game/RPG_InventorySystem/Blueprints/SaveSystem/Meta_SaveGame.Meta_SaveGame_C|GetSlotNames _metasave))
  ;[0 1 0.498 0.201] Load Most Recent Save
  (Utilities|FlowControl|Delay 0.0)
  (CallFunction|LoadData (Utilities|Array|Get(acopy) _slotnames (Utilities|Array|LastIndex _slotnames))))