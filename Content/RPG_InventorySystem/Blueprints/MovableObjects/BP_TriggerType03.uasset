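; Interactable rotating trigger that turns its mesh by a yaw step on each use and notifies an associated actor.
; ACInteractable handles the interaction area, widget, five highlightable meshes and the stored value that Interaction changes.
; A timeline lerps yaw by RotationValue, saves the resulting rotation, then optionally reinitializes the interactable.
; On game load, the rotation is rebuilt from InteractableValue times RotationValue.
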(event Custom|Move%20Forward
  ;[1 0.02708 0 0.18] Moving Animation
  (Variables|/Game/RPG_InventorySystem/Blueprints/Components/AC_Interactable.AC_Interactable_C|SetTimeline%20Direction (Variables|Default|GetAC_Interactable) "Forward")
  (bind _newtrack_0 (Timeline|Timeline_0 PlayFromStart)
    (:Update
      (Transformation|SetRelativeRotation (Variables|Default|GetStaticMesh) (Math|Rotator|Lerp(Rotator) (Variables|Default|GetCurrentRotation) (Math|Rotator|MakeRotator (.Roll (Math|Rotator|BreakRotator (Variables|Default|GetCurrentRotation))) (.Pitch (Math|Rotator|BreakRotator (Variables|Default|GetCurrentRotation))) (+ (.Yaw (Math|Rotator|BreakRotator (Variables|Default|GetCurrentRotation))) (Variables|Default|GetRotation%20Value))) _newtrack_0) false false))
    (:Finished
      (Variables|Default|SetCurrentRotation (Variables|/Script/Engine.SceneComponent|GetRelativeRotation (Variables|Default|GetStaticMesh)))
      (if (Variables|Default|GetRe-initialize%20on%20Moving%20Finished)
        (Default|EventRe-initialize (Variables|Default|GetAC_Interactable))))))

(event Custom|Move%20Backward
  ;[1 0.02708 0 0.18] Moving Animation
  (Variables|/Game/RPG_InventorySystem/Blueprints/Components/AC_Interactable.AC_Interactable_C|SetTimeline%20Direction (Variables|Default|GetAC_Interactable) "Backward")
  (bind _newtrack_0 (Timeline|Timeline_0 ReverseFromEnd)
    (:Update
      (Transformation|SetRelativeRotation (Variables|Default|GetStaticMesh) (Math|Rotator|Lerp(Rotator) (Variables|Default|GetCurrentRotation) (Math|Rotator|MakeRotator (.Roll (Math|Rotator|BreakRotator (Variables|Default|GetCurrentRotation))) (.Pitch (Math|Rotator|BreakRotator (Variables|Default|GetCurrentRotation))) (+ (.Yaw (Math|Rotator|BreakRotator (Variables|Default|GetCurrentRotation))) (Variables|Default|GetRotation%20Value))) _newtrack_0) false false))
    (:Finished
      (Variables|Default|SetCurrentRotation (Variables|/Script/Engine.SceneComponent|GetRelativeRotation (Variables|Default|GetStaticMesh)))
      (if (Variables|Default|GetRe-initialize%20on%20Moving%20Finished)
        (Default|EventRe-initialize (Variables|Default|GetAC_Interactable))))))

(event EventInteraction
  ;[0 0 0 0.227 22] On Interaction
  (Default|ChangeInteractableValue (Variables|Default|GetAC_Interactable) true)
  (Default|EventAssociatedActorInteraction (Variables|Default|GetAC_Interactable))
  (CallFunction|MoveForward))

(event EventInitialize
  ;[0 0 0 0.227 22] On Initialize
  (Default|SetupInteractableReferences (Variables|Default|GetAC_Interactable) (Variables|Default|GetInteractableArea) (Variables|Default|GetInteractionWidget) (Utilities|Set|MakeSet (Variables|Default|GetStaticMesh) (Variables|Default|GetStaticMesh1) (Variables|Default|GetStaticMesh2) (Variables|Default|GetStaticMesh3) (Variables|Default|GetStaticMesh4))))

(event EventRemoveInteraction
  ;[0 0 0 0.227 22] On Remove Interaction
)

(event EventGameLoad
  (bind _ac_interactable (Variables|Default|GetAC_Interactable))
  (bind _interactable_value (Variables|/Game/RPG_InventorySystem/Blueprints/Components/AC_Interactable.AC_Interactable_C|GetInteractable%20Value _ac_interactable))
  ;[0 0 0 0.227 22] On Game Load
  (if (!= _interactable_value 0)
    (bind _output_get (Variables|Default|SetCurrentRotation (Math|Rotator|MakeRotator 0.0 0.0 (* _interactable_value (Variables|Default|GetRotation%20Value)))))
    (Transformation|SetRelativeRotation (Variables|Default|GetStaticMesh) _output_get false false)
    (else
      (bind _output_get_2 (Variables|Default|SetCurrentRotation "0, 0, 0"))
      (Transformation|SetRelativeRotation (Variables|Default|GetStaticMesh) _output_get_2 false false))))

(event EventEndInteraction
  ;[0 0 0 0.227 22] On End Interaction
)

(fn ConstructionScript)