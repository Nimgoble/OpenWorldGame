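; Ambient audio Blueprint that crossfades between a day sound and a night sound in step with BP_DayNightCycle.
; On BeginPlay it binds to the first cycle actor's day and night triggers and sets initial volumes from the time of day, or starts a one-second timer if none exists.
; The AudioBlend timeline, rate-scaled by AudioBlendTime, plays or reverses to drive the two volumes inversely.
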(event Custom|BindAudioTriggers
  (bind _outactors (Actor|GetAllActorsOfClass "/Game/DayNightCycle/Blueprints/BP_DayNightCycle.BP_DayNightCycle_C"))
  (if (> (Utilities|Array|Length _outactors) 0)
    (EventDispatchers|BindEventtoTriggerDay (Utilities|Array|Get(acopy) _outactors) (EventDispatchers|CreateEvent :!event TriggerDayAudio))
    (EventDispatchers|BindEventtoTriggerNight (Utilities|Array|Get(acopy) _outactors) (EventDispatchers|CreateEvent :!event TriggerNightAudio))
    (bind _timeoftheday (Default|DetermineNightorDayTime (Utilities|Array|Get(acopy) _outactors)))
    (CallFunction|Initialize (Utilities|Select :Index _timeoftheday :Option%200 false :Option%201 true))
    (else
      (Utilities|Time|SetTimerbyEvent (EventDispatchers|CreateEvent :!event Custom|BindAudioTriggers) 1.0))))

(event EventBeginPlay
  (CallFunction|SetSounds)
  (Components|Timeline|SetPlayRate (Variables|Default|GetAudioBlend) (/ 1.0 (Variables|Default|GetAudioBlendTime)))
  (CallFunction|BindAudioTriggers))

(fn ConstructionScript
  (CallFunction|SetSounds))

(fn TriggerNightAudio
  (Utilities|String|Reverse (Variables|Default|GetAudioBlend)))

(fn TriggerDayAudio
  (Audio|Components|Audio|Play (Variables|Default|GetAudioBlend)))

(fn SetSounds
  (Audio|Components|Audio|SetSound (Variables|Default|GetAudioNight) (Variables|Default|GetNightSound))
  (Audio|Components|Audio|SetSound (Variables|Default|GetAudioDay) (Variables|Default|GetDaySound)))

(fn Initialize
  (params (DaySound :type Boolean))
  (bind _returnvalue (select DaySound 1.0 0.0))
  (Audio|Components|Audio|SetVolumeMultiplier (Variables|Default|GetAudioNight) (- 1.0 _returnvalue) :!class /Script/Engine.AudioComponent)
  (Audio|Components|Audio|SetVolumeMultiplier (Variables|Default|GetAudioDay) _returnvalue :!class /Script/Engine.AudioComponent))