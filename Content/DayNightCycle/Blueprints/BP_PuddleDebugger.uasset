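; Debug actor that visualizes what BP_DayNightCycle captures for puddles, on begin play and optionally on a repeating timer.
; For the locally controlled player, it draws position-colored boxes and size labels around each non-ignored captured asset.
; Bounds optionally come from merged component bounds, skipping frustum components.
; It also prints the Z extremes, boxes the combined bounds in red, and briefly repurposes the cycle's scene capture to render base color into DepthBuffer_RGB.
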(event EventBeginPlay
  (if (Variables|Default|GetbEnabled)
    (Utilities|FlowControl|Delay (Variables|Default|GetStartDelay))
    (CallFunction|DebugPuddles)
    (if (> (Variables|Default|GetRegenerateTime) 0.0)
      (Utilities|Time|SetTimerbyEvent (EventDispatchers|CreateEvent :!event DebugPuddles) (Variables|Default|GetRegenerateTime) true))))

(event Collision|EventActorBeginOverlap
  (params (OtherActor :type Actor%20Object%20Reference)))

(fn ConstructionScript)

(fn DebugPuddles
  (bind _returnvalue (Game|Player|GetPlayerPawn 0))
  (bind _regeneratetime (Variables|Default|GetRegenerateTime))
  (if (Variables|Default|GetbEnabled)
    (Components|DestroyComponent (Actor|GetComponentsByClass "/Script/Engine.TextRenderComponent"))
    (Utilities|IsValid _returnvalue
      (:Is%20Valid
        (if (Pawn|IsLocallyControlled _returnvalue)
          (bind _outactors (Actor|GetAllActorsOfClass "/Game/DayNightCycle/Blueprints/BP_DayNightCycle.BP_DayNightCycle_C"))
          (for _array_element _outactors
            (LocalVariables|SetL_DayNightCycle _array_element)
            (for _array_element_2 (Variables|/Game/DayNightCycle/Blueprints/BP_DayNightCycle.BP_DayNightCycle_C|GetAssetsToCapture (LocalVariables|GetL_DayNightCycle))
              (bind _output_get (LocalVariables|SetL_Actor _array_element_2))
              (Utilities|IsValid _output_get
                (:Is%20Valid
                  (if (== (Utilities|Array|FindItem (Variables|Default|GetClassesToIgnoreForDebugging) (Utilities|GetClass _array_element_2)) -1)
                    (if (Math|Boolean|ANDBoolean (!= (.X (Math|Vector|BreakVector (* (.boxextent (select (Variables|/Game/DayNightCycle/Blueprints/BP_DayNightCycle.BP_DayNightCycle_C|GetbUseAccurateBoundsCalculation (LocalVariables|GetL_DayNightCycle)) (CallFunction|BoundsCalculationFunc (LocalVariables|GetL_Actor)) (Utilities|Struct|MakeBoxSphereBounds (.Origin (Collision|GetActorBounds (LocalVariables|GetL_Actor) false)) (.BoxExtent (Collision|GetActorBounds (LocalVariables|GetL_Actor) false)) 0.0))) 2))) 0.0) (!= (.Y (Math|Vector|BreakVector (* (.boxextent (select (Variables|/Game/DayNightCycle/Blueprints/BP_DayNightCycle.BP_DayNightCycle_C|GetbUseAccurateBoundsCalculation (LocalVariables|GetL_DayNightCycle)) (CallFunction|BoundsCalculationFunc (LocalVariables|GetL_Actor)) (Utilities|Struct|MakeBoxSphereBounds (.Origin (Collision|GetActorBounds (LocalVariables|GetL_Actor) false)) (.BoxExtent (Collision|GetActorBounds (LocalVariables|GetL_Actor) false)) 0.0))) 2))) 0.0) (!= (.Z (Math|Vector|BreakVector (* (.boxextent (select (Variables|/Game/DayNightCycle/Blueprints/BP_DayNightCycle.BP_DayNightCycle_C|GetbUseAccurateBoundsCalculation (LocalVariables|GetL_DayNightCycle)) (CallFunction|BoundsCalculationFunc (LocalVariables|GetL_Actor)) (Utilities|Struct|MakeBoxSphereBounds (.Origin (Collision|GetActorBounds (LocalVariables|GetL_Actor) false)) (.BoxExtent (Collision|GetActorBounds (LocalVariables|GetL_Actor) false)) 0.0))) 2))) 0.0))
                      (Utilities|FlowControl|Sequence
                        (:then_0
                          (if (>= (.Z (Math|Vector|BreakVector (+ (.origin (select (Variables|/Game/DayNightCycle/Blueprints/BP_DayNightCycle.BP_DayNightCycle_C|GetbUseAccurateBoundsCalculation (LocalVariables|GetL_DayNightCycle)) (CallFunction|BoundsCalculationFunc (LocalVariables|GetL_Actor)) (Utilities|Struct|MakeBoxSphereBounds (.Origin (Collision|GetActorBounds (LocalVariables|GetL_Actor) false)) (.BoxExtent (Collision|GetActorBounds (LocalVariables|GetL_Actor) false)) 0.0))) (.boxextent (select (Variables|/Game/DayNightCycle/Blueprints/BP_DayNightCycle.BP_DayNightCycle_C|GetbUseAccurateBoundsCalculation (LocalVariables|GetL_DayNightCycle)) (CallFunction|BoundsCalculationFunc (LocalVariables|GetL_Actor)) (Utilities|Struct|MakeBoxSphereBounds (.Origin (Collision|GetActorBounds (LocalVariables|GetL_Actor) false)) (.BoxExtent (Collision|GetActorBounds (LocalVariables|GetL_Actor) false)) 0.0)))))) (Variables|Default|GetMaxZ))
                            (Variables|Default|SetMaxZ (.Z (Math|Vector|BreakVector (+ (.origin (select (Variables|/Game/DayNightCycle/Blueprints/BP_DayNightCycle.BP_DayNightCycle_C|GetbUseAccurateBoundsCalculation (LocalVariables|GetL_DayNightCycle)) (CallFunction|BoundsCalculationFunc (LocalVariables|GetL_Actor)) (Utilities|Struct|MakeBoxSphereBounds (.Origin (Collision|GetActorBounds (LocalVariables|GetL_Actor) false)) (.BoxExtent (Collision|GetActorBounds (LocalVariables|GetL_Actor) false)) 0.0))) (.boxextent (select (Variables|/Game/DayNightCycle/Blueprints/BP_DayNightCycle.BP_DayNightCycle_C|GetbUseAccurateBoundsCalculation (LocalVariables|GetL_DayNightCycle)) (CallFunction|BoundsCalculationFunc (LocalVariables|GetL_Actor)) (Utilities|Struct|MakeBoxSphereBounds (.Origin (Collision|GetActorBounds (LocalVariables|GetL_Actor) false)) (.BoxExtent (Collision|GetActorBounds (LocalVariables|GetL_Actor) false)) 0.0)))))))
                            (Variables|Default|SetMaxZName (Utilities|GetDisplayName (LocalVariables|GetL_Actor)))))
                        (:then_1
                          (if (<= (.Z (Math|Vector|BreakVector (- (.origin (select (Variables|/Game/DayNightCycle/Blueprints/BP_DayNightCycle.BP_DayNightCycle_C|GetbUseAccurateBoundsCalculation (LocalVariables|GetL_DayNightCycle)) (CallFunction|BoundsCalculationFunc (LocalVariables|GetL_Actor)) (Utilities|Struct|MakeBoxSphereBounds (.Origin (Collision|GetActorBounds (LocalVariables|GetL_Actor) false)) (.BoxExtent (Collision|GetActorBounds (LocalVariables|GetL_Actor) false)) 0.0))) (.boxextent (select (Variables|/Game/DayNightCycle/Blueprints/BP_DayNightCycle.BP_DayNightCycle_C|GetbUseAccurateBoundsCalculation (LocalVariables|GetL_DayNightCycle)) (CallFunction|BoundsCalculationFunc (LocalVariables|GetL_Actor)) (Utilities|Struct|MakeBoxSphereBounds (.Origin (Collision|GetActorBounds (LocalVariables|GetL_Actor) false)) (.BoxExtent (Collision|GetActorBounds (LocalVariables|GetL_Actor) false)) 0.0)))))) (Variables|Default|GetMinZ))
                            (Variables|Default|SetMinZ (.Z (Math|Vector|BreakVector (- (.origin (select (Variables|/Game/DayNightCycle/Blueprints/BP_DayNightCycle.BP_DayNightCycle_C|GetbUseAccurateBoundsCalculation (LocalVariables|GetL_DayNightCycle)) (CallFunction|BoundsCalculationFunc (LocalVariables|GetL_Actor)) (Utilities|Struct|MakeBoxSphereBounds (.Origin (Collision|GetActorBounds (LocalVariables|GetL_Actor) false)) (.BoxExtent (Collision|GetActorBounds (LocalVariables|GetL_Actor) false)) 0.0))) (.boxextent (select (Variables|/Game/DayNightCycle/Blueprints/BP_DayNightCycle.BP_DayNightCycle_C|GetbUseAccurateBoundsCalculation (LocalVariables|GetL_DayNightCycle)) (CallFunction|BoundsCalculationFunc (LocalVariables|GetL_Actor)) (Utilities|Struct|MakeBoxSphereBounds (.Origin (Collision|GetActorBounds (LocalVariables|GetL_Actor) false)) (.BoxExtent (Collision|GetActorBounds (LocalVariables|GetL_Actor) false)) 0.0)))))))
                            (Variables|Default|SetMinZName (Utilities|GetDisplayName (LocalVariables|GetL_Actor)))))
                        (:then_2
                          (bind _output_get_2 (LocalVariables|SetTextColor (Utilities|Struct|MakeLinearColor (Math|Float|Fraction (.x (Transformation|GetActorLocation (LocalVariables|GetL_Actor)))) (Math|Float|Fraction (.y (Transformation|GetActorLocation (LocalVariables|GetL_Actor)))) (Math|Float|Fraction (.z (Transformation|GetActorLocation (LocalVariables|GetL_Actor)))) 1.0)))
                          (Rendering|Debug|DrawDebugBox (.origin (select (Variables|/Game/DayNightCycle/Blueprints/BP_DayNightCycle.BP_DayNightCycle_C|GetbUseAccurateBoundsCalculation (LocalVariables|GetL_DayNightCycle)) (CallFunction|BoundsCalculationFunc (LocalVariables|GetL_Actor)) (Utilities|Struct|MakeBoxSphereBounds (.Origin (Collision|GetActorBounds (LocalVariables|GetL_Actor) false)) (.BoxExtent (Collision|GetActorBounds (LocalVariables|GetL_Actor) false)) 0.0))) (.boxextent (select (Variables|/Game/DayNightCycle/Blueprints/BP_DayNightCycle.BP_DayNightCycle_C|GetbUseAccurateBoundsCalculation (LocalVariables|GetL_DayNightCycle)) (CallFunction|BoundsCalculationFunc (LocalVariables|GetL_Actor)) (Utilities|Struct|MakeBoxSphereBounds (.Origin (Collision|GetActorBounds (LocalVariables|GetL_Actor) false)) (.BoxExtent (Collision|GetActorBounds (LocalVariables|GetL_Actor) false)) 0.0))) _output_get_2 "0, 0, 0" (select (> _regeneratetime 0.0) _regeneratetime 999999.0) (Variables|Default|GetDebugBoxesThickness))
                          (bind _returnvalue_2 (AddComponent|AddTextRenderComponent false))
                          (Transformation|SetWorldLocation _returnvalue_2 (+ (.origin (select (Variables|/Game/DayNightCycle/Blueprints/BP_DayNightCycle.BP_DayNightCycle_C|GetbUseAccurateBoundsCalculation (LocalVariables|GetL_DayNightCycle)) (CallFunction|BoundsCalculationFunc (LocalVariables|GetL_Actor)) (Utilities|Struct|MakeBoxSphereBounds (.Origin (Collision|GetActorBounds (LocalVariables|GetL_Actor) false)) (.BoxExtent (Collision|GetActorBounds (LocalVariables|GetL_Actor) false)) 0.0))) (.boxextent (select (Variables|/Game/DayNightCycle/Blueprints/BP_DayNightCycle.BP_DayNightCycle_C|GetbUseAccurateBoundsCalculation (LocalVariables|GetL_DayNightCycle)) (CallFunction|BoundsCalculationFunc (LocalVariables|GetL_Actor)) (Utilities|Struct|MakeBoxSphereBounds (.Origin (Collision|GetActorBounds (LocalVariables|GetL_Actor) false)) (.BoxExtent (Collision|GetActorBounds (LocalVariables|GetL_Actor) false)) 0.0)))) false false)
                          (Rendering|Components|TextRender|SetText _returnvalue_2 (Utilities|Text|ToText(String) (Utilities|String|Append (Utilities|GetDisplayName (LocalVariables|GetL_Actor)) " X: " (Utilities|String|ToString(Integer) (Math|Float|Floor (.X (Math|Vector|BreakVector (* (.boxextent (select (Variables|/Game/DayNightCycle/Blueprints/BP_DayNightCycle.BP_DayNightCycle_C|GetbUseAccurateBoundsCalculation (LocalVariables|GetL_DayNightCycle)) (CallFunction|BoundsCalculationFunc (LocalVariables|GetL_Actor)) (Utilities|Struct|MakeBoxSphereBounds (.Origin (Collision|GetActorBounds (LocalVariables|GetL_Actor) false)) (.BoxExtent (Collision|GetActorBounds (LocalVariables|GetL_Actor) false)) 0.0))) 2))))) " Y: " (Utilities|String|ToString(Integer) (Math|Float|Floor (.Y (Math|Vector|BreakVector (* (.boxextent (select (Variables|/Game/DayNightCycle/Blueprints/BP_DayNightCycle.BP_DayNightCycle_C|GetbUseAccurateBoundsCalculation (LocalVariables|GetL_DayNightCycle)) (CallFunction|BoundsCalculationFunc (LocalVariables|GetL_Actor)) (Utilities|Struct|MakeBoxSphereBounds (.Origin (Collision|GetActorBounds (LocalVariables|GetL_Actor) false)) (.BoxExtent (Collision|GetActorBounds (LocalVariables|GetL_Actor) false)) 0.0))) 2))))) " Z: " (Utilities|String|ToString(Integer) (Math|Float|Floor (.Z (Math|Vector|BreakVector (* (.boxextent (select (Variables|/Game/DayNightCycle/Blueprints/BP_DayNightCycle.BP_DayNightCycle_C|GetbUseAccurateBoundsCalculation (LocalVariables|GetL_DayNightCycle)) (CallFunction|BoundsCalculationFunc (LocalVariables|GetL_Actor)) (Utilities|Struct|MakeBoxSphereBounds (.Origin (Collision|GetActorBounds (LocalVariables|GetL_Actor) false)) (.BoxExtent (Collision|GetActorBounds (LocalVariables|GetL_Actor) false)) 0.0))) 2))))))))
                          (Class|TextRenderComponent|SetTextMaterial _returnvalue_2 "/Engine/EngineMaterials/UnlitText.UnlitText")
                          (Rendering|Components|TextRender|SetTextRenderColor _returnvalue_2 (Math|Conversions|ToColor(LinearColor) (LocalVariables|GetTextColor))))))))))
            (Development|PrintString (Utilities|String|Append "MaxZ: " (Variables|Default|GetMaxZName) " at " (Utilities|String|ToString(Float) (Variables|Default|GetMaxZ))) true true "(R=0.000000,G=0.660000,B=1.000000,A=1.000000)" 2e+01)
            (Development|PrintString (Utilities|String|Append "MinZ: " (Variables|Default|GetMinZName) " at " (Utilities|String|ToString(Float) (Variables|Default|GetMinZ))) true true "(R=0.000000,G=0.660000,B=1.000000,A=1.000000)" 2e+01)
            (if (Variables|/Game/DayNightCycle/Blueprints/BP_DayNightCycle.BP_DayNightCycle_C|GetbUseAccurateBoundsCalculation (LocalVariables|GetL_DayNightCycle))
              (bind _bounds (Default|CalculateAccurateBounds (LocalVariables|GetL_DayNightCycle) (Variables|/Game/DayNightCycle/Blueprints/BP_DayNightCycle.BP_DayNightCycle_C|GetAssetsToCapture (LocalVariables|GetL_DayNightCycle))))
              (LocalVariables|SetL_Bounds _bounds)
              (else
                (bind (_center _boxextent) (Collision|GetActorArrayBounds (Variables|/Game/DayNightCycle/Blueprints/BP_DayNightCycle.BP_DayNightCycle_C|GetAssetsToCapture (LocalVariables|GetL_DayNightCycle))))
                (LocalVariables|SetL_Bounds (Utilities|Struct|MakeBoxSphereBounds _center _boxextent 0.0))))
            (Rendering|Debug|DrawDebugBox (.origin (LocalVariables|GetL_Bounds)) (.boxextent (LocalVariables|GetL_Bounds)) "(R=1.000000,G=0.000000,B=0.000000,A=1.000000)" "0, 0, 0" (Math|Float|Min(Float) (Variables|Default|GetRegenerateTime) 2e+01) 5e+01)
            (Variables|/Script/Engine.SceneCaptureComponent2D|SetCaptureSource (Variables|/Game/DayNightCycle/Blueprints/BP_DayNightCycle.BP_DayNightCycle_C|GetSceneCaptureComponent2D (LocalVariables|GetL_DayNightCycle)) "SCS_BaseColor")
            (LocalVariables|SetL_TextureTarget (Variables|/Script/Engine.SceneCaptureComponent2D|GetTextureTarget (Variables|/Game/DayNightCycle/Blueprints/BP_DayNightCycle.BP_DayNightCycle_C|GetSceneCaptureComponent2D (LocalVariables|GetL_DayNightCycle))))
            (Variables|/Script/Engine.SceneCaptureComponent2D|SetTextureTarget (Variables|/Game/DayNightCycle/Blueprints/BP_DayNightCycle.BP_DayNightCycle_C|GetSceneCaptureComponent2D (LocalVariables|GetL_DayNightCycle)) "/Game/DayNightCycle/Textures/DepthBuffer_RGB.DepthBuffer_RGB")
            (Rendering|SceneCapture|CaptureScene (Variables|/Game/DayNightCycle/Blueprints/BP_DayNightCycle.BP_DayNightCycle_C|GetSceneCaptureComponent2D (LocalVariables|GetL_DayNightCycle)) :!class /Script/Engine.SceneCaptureComponent2D)
            (Variables|/Script/Engine.SceneCaptureComponent2D|SetTextureTarget (Variables|/Game/DayNightCycle/Blueprints/BP_DayNightCycle.BP_DayNightCycle_C|GetSceneCaptureComponent2D (LocalVariables|GetL_DayNightCycle)) (LocalVariables|GetL_TextureTarget))
            (Variables|/Script/Engine.SceneCaptureComponent2D|SetCaptureSource (Variables|/Game/DayNightCycle/Blueprints/BP_DayNightCycle.BP_DayNightCycle_C|GetSceneCaptureComponent2D (LocalVariables|GetL_DayNightCycle)) "SCS_SceneDepth")))))))

(fn BoundsCalculationFunc
  (params (Actor :type Actor%20Object%20Reference))
  (bind _output_get (LocalVariables|SetB_Max (Transformation|GetActorLocation Actor)))
  (LocalVariables|SetB_Min _output_get)
  (for _array_element (Actor|GetComponentsByClass Actor "/Script/Engine.SceneComponent")
    (if (not (== (Utilities|GetClass _array_element) "/Script/Engine.DrawFrustumComponent"))
      (Utilities|FlowControl|Sequence
        (:then_0
          (LocalVariables|SetB_Max (Math|Vector|MakeVector (Math|Float|Max(Float) (.x (LocalVariables|GetB_Max)) (.x (+ (.Origin (Collision|GetComponentBounds _array_element)) (.BoxExtent (Collision|GetComponentBounds _array_element))))) (Math|Float|Max(Float) (.y (LocalVariables|GetB_Max)) (.y (+ (.Origin (Collision|GetComponentBounds _array_element)) (.BoxExtent (Collision|GetComponentBounds _array_element))))) (Math|Float|Max(Float) (.z (LocalVariables|GetB_Max)) (.z (+ (.Origin (Collision|GetComponentBounds _array_element)) (.BoxExtent (Collision|GetComponentBounds _array_element))))))))
        (:then_1
          (LocalVariables|SetB_Min (Math|Vector|MakeVector (Math|Float|Min(Float) (.x (LocalVariables|GetB_Min)) (.x (- (.Origin (Collision|GetComponentBounds _array_element)) (.BoxExtent (Collision|GetComponentBounds _array_element))))) (Math|Float|Min(Float) (.y (LocalVariables|GetB_Min)) (.y (- (.Origin (Collision|GetComponentBounds _array_element)) (.BoxExtent (Collision|GetComponentBounds _array_element))))) (Math|Float|Min(Float) (.z (LocalVariables|GetB_Min)) (.z (- (.Origin (Collision|GetComponentBounds _array_element)) (.BoxExtent (Collision|GetComponentBounds _array_element)))))))))))
  (return (Utilities|Struct|MakeBoxSphereBounds (+ (/ (- (LocalVariables|GetB_Max) (LocalVariables|GetB_Min)) 2.0) (LocalVariables|GetB_Min)) (/ (- (LocalVariables|GetB_Max) (LocalVariables|GetB_Min)) 2.0) 0.0)))